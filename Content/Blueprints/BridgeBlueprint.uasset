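; Physics-driven bridge that strings simulated ring meshes along the BridgeExtents spline.
; The construction script spawns the rings and collision-disabling physics constraints by distance along the spline, and moves Beginning and End to its first two points.
; Tick links one neighboring ring pair per frame through an unbounded counter.
; It also adds new physics handles every frame to grab the first and last rings at Beginning and End.
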(event EventTick
  (params (DeltaSeconds :type Float%20%28single-precision%29))
  (bind _boxes (Variables|Default|GetBoxes))
  (Utilities|FlowControl|Sequence
    (:then_0
      (bind _returnvalue (AddComponent|AddPhysicsHandleComponent false))
      (Class|PhysicsHandleComponent|GrabComponent _returnvalue (Utilities|Array|Get(acopy) _boxes) "None" (Transformation|GetWorldLocation (Variables|Default|GetBeginning)) false))
    (:then_1
      (bind _returnvalue_2 (AddComponent|AddPhysicsHandleComponent false))
      (Class|PhysicsHandleComponent|GrabComponent _returnvalue_2 (Utilities|Array|Get(acopy) _boxes (Utilities|Array|LastIndex _boxes)) "None" (Transformation|GetWorldLocation (Variables|Default|GetEnd)) false))
    (:then_2
      (Class|PhysicsConstraintComponent|SetConstrainedComponents (Utilities|Array|Get(acopy) (Variables|Default|GetPhysicsHooks) (Variables|Default|GetLastNumber)) (Utilities|Array|Get(acopy) _boxes (Variables|Default|GetLastNumber)) "None" (Utilities|Array|Get(acopy) _boxes (+ (Variables|Default|GetLastNumber) 1)) "None")
      (Variables|Default|SetLastNumber (+ (Variables|Default|GetLastNumber) 1)))))

(fn ConstructionScript
  (bind _boxes (Variables|Default|GetBoxes))
  (bind _bridgeextents (Variables|Default|GetBridgeExtents))
  (Utilities|FlowControl|Sequence
    (:then_0
      (Utilities|FlowControl|DoOnce false
        (:Completed
          (for _index (range 0 (.ReturnValue (Math|Float|Division(WholeandRemainder) (Spline|GetSplineLength _bridgeextents) 32.0)))
            (bind _returnvalue (AddComponent|AddStaticMeshComponent false))
            (bind _returnvalue_2 (Utilities|Array|Add _boxes _returnvalue))
            (Components|StaticMesh|SetStaticMesh (Utilities|Array|Get(acopy) _boxes _returnvalue_2) "/Game/Objects/Ring.Ring")
            (Transformation|SetWorldLocation (Utilities|Array|Get(acopy) _boxes _returnvalue_2) (Class|SplineComponent|GetWorldLocationatDistanceAlongSpline _bridgeextents (* _index 64.0)) false)
            (Collision|SetCollisionObjectType (Utilities|Array|Get(acopy) _boxes _returnvalue_2) "ECC_GameTraceChannel5")
            (Collision|SetCollisionEnabled (Utilities|Array|Get(acopy) _boxes _returnvalue_2) "QueryAndPhysics")
            (Physics|SetSimulatePhysics (Utilities|Array|Get(acopy) _boxes _returnvalue_2) true)
            (bind _returnvalue_3 (AddComponent|AddPhysicsConstraintComponent false))
            (Utilities|Array|Add (Variables|Default|GetPhysicsHooks) _returnvalue_3)
            (Transformation|SetWorldLocation _returnvalue_3 (Class|SplineComponent|GetWorldLocationatDistanceAlongSpline _bridgeextents (* _index 64.0)) false)
            (Class|PhysicsConstraintComponent|SetDisableCollision _returnvalue_3 true)
            (Transformation|SetWorldLocation (Variables|Default|GetBeginning) (Class|SplineComponent|GetWorldLocationatSplinePoint (Variables|Default|GetBridgeExtents)) false)
            (Transformation|SetWorldLocation (Variables|Default|GetEnd) (Class|SplineComponent|GetWorldLocationatSplinePoint (Variables|Default|GetBridgeExtents) 1) false)))))))