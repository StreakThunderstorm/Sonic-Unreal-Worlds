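; HUD Blueprint for a Sonic-style game that prepares the digits for rings, lives and a minutes-and-seconds timer.
; BeginPlay caches the SUWGameInstance and creates a SUWHUDWidget.
; Tick converts game time to milliseconds in Gametimer.
; DrawHUD splits BP_Character's held rings, the game instance's lives and the timer into single-digit variables using division and modulo, with minutes wrapping every ten.
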(event EventDrawHUD
  (params (SizeX :type Integer) (SizeY :type Integer))
  (bind _gametimer (Variables|Default|GetGametimer))
  (bind _gametimer_2 (Variables|Default|GetGametimer))
  (bind _gameinstance (Variables|Default|GetGameInstance))
  (bind _returnvalue (/ _gametimer 1e+03))
  (bind _returnvalue_2 (/ _gametimer_2 6e+04))
  (bind _lives (Variables|/Game/Blueprints/SUWGameInstance.SUWGameInstance_C|GetLives _gameinstance))
  (bind _returnvalue_3 (Math|Float|%(Float) _returnvalue 6e+01))
  (bind _returnvalue_4 (Math|Float|%(Float) _returnvalue_2 1e+01))
  (bind _returnvalue_5 (Math|Float|Floor _returnvalue_3))
  (bind _returnvalue_6 (Math|Float|Floor _returnvalue_4))
  (Utilities|FlowControl|Sequence
    (:then_0
      (bind _asbp_character (Utilities|Casting|CastToBP_Character (Game|Player|GetPlayerPawn 0)))
      (Utilities|FlowControl|Sequence
        (:then_0
          (Variables|Default|SetRingsOnes (Math|Integer|%(Integer) (Variables|/Game/Blueprints/BP_Character.BP_Character_C|GetHeldRings _asbp_character) 10))
          (Variables|Default|SetRingsTens (Math|Integer|%(Integer) (/ (Variables|/Game/Blueprints/BP_Character.BP_Character_C|GetHeldRings _asbp_character) 10) 10))
          (Variables|Default|SetRingsHundreds (Math|Integer|%(Integer) (/ (Variables|/Game/Blueprints/BP_Character.BP_Character_C|GetHeldRings _asbp_character) 100) 10)))
        (:then_1
          (Variables|Default|SetLivesOnes (Math|Integer|%(Integer) _lives 10))
          (Variables|Default|SetLivesTens (Math|Integer|%(Integer) (/ _lives 10) 10)))))
    (:then_1
      (Utilities|FlowControl|Sequence
        (:then_0
          (Variables|Default|SetSecondTens (Math|Integer|%(Integer) (/ _returnvalue_5 10) 10))
          (Variables|Default|SetSecondOnes (Math|Integer|%(Integer) _returnvalue_5 10)))
        (:then_1
          (Variables|Default|SetMinuteTens (Math|Integer|%(Integer) (/ _returnvalue_6 10) 10))
          (Variables|Default|SetMinuteOnes (Math|Integer|%(Integer) _returnvalue_6 10)))))))

(event EventTick
  (params (DeltaSeconds :type Float%20%28single-precision%29))
  (Variables|Default|SetGametimer (* (Utilities|Time|GetGameTimeinSeconds) 1e+03)))

(event EventBeginPlay
  (bind _assuwgame_instance (Utilities|Casting|CastToSUWGameInstance (Game|GetGameInstance)))
  (Variables|Default|SetGameInstance _assuwgame_instance)
  (UserInterface|CreateWidget "/Game/Blueprints/SUWHUDWidget.SUWHUDWidget_C"))

(fn ConstructionScript)