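; BP_Ring is a spinning ring pickup that homes in on the player while shield type 2 is active.
; Tick pulls nearby rings with distance-scaled, clamped acceleration and frame-time-scaled movement, adding a sine wobble.
; Losing that shield turns attracted rings into dropped physics bodies that keep their velocity and cannot be re-attracted.
; Moving rings become obtainable after a short delay, then flicker and destroy themselves.
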(event EventBeginPlay
  (bind _asbp_character (Utilities|Casting|CastToBP_Character (Game|Player|GetPlayerPawn 0)))
  (Variables|Default|SetPlayer _asbp_character))

(event EventTick
  (params (DeltaSeconds :type Float%20%28single-precision%29))
  (bind _returnvalue (Transformation|GetActorLocation))
  (bind _ringmesh (Variables|Actor|GetRingMesh))
  (bind _collision (Variables|Default|GetCollision))
  (bind _player (Variables|Default|GetPlayer))
  (bind _returnvalue_2 (Transformation|GetWorldRotation _ringmesh))
  (bind _returnvalue_3 (Transformation|GetActorLocation _player))
  (bind (_roll _pitch _yaw) (Math|Rotator|BreakRotator _returnvalue_2))
  (bind _returnvalue_4 (- _returnvalue_3 _returnvalue))
  (Variables|Default|SetDeltaTime (/ DeltaSeconds 0.016))
  (Utilities|FlowControl|Sequence
    (:then_0
      (Utilities|FlowControl|Sequence
        (:then_0
          (Transformation|SetWorldRotation _ringmesh (Math|Rotator|MakeRotator _roll _pitch (+ _yaw 5.0)) false false))
        (:then_1
          (if (Variables|Default|GetMoving)
            (Utilities|FlowControl|Sequence
              (:then_0
                (Class|PrimitiveComponent|WakeAllRigidBodies (Variables|Default|GetCollision))
                (Utilities|FlowControl|Delay 1.0)
                (Variables|Default|SetObtainable true)
                (Utilities|FlowControl|Delay 3.0)
                (Variables|Default|SetFading true)
                (Utilities|FlowControl|Delay 2.0)
                (Actor|DestroyActor))
              (:then_1
                (if (Variables|Default|GetFading)
                  (Utilities|FlowControl|Delay 0.1)
                  (Rendering|ToggleVisibility (Variables|Actor|GetRingMesh) false))))))))
    (:then_1
      (if (Variables|Default|GetAttracted)
        (Utilities|FlowControl|Sequence
          (:then_0
            ;[1 1 1] Calculate Attracted Speed
            (bind _output_get (Variables|Default|SetSpeed (+ (Variables|Default|GetSpeed) (* (* _returnvalue_4 (* (Variables|Default|GetDeltaTime) (Variables|Default|GetAcceleration))) (Math|Vector|VectorLength _returnvalue_4)))))
            (Variables|Default|SetSpeed (Math|Vector|ClampVectorSize _output_get (* (Variables|Default|GetMaxSpeed) -1.0) (Variables|Default|GetMaxSpeed))))
          (:then_1
            ;[1 1 1] Move Attracted Ring
            (Transformation|SetActorLocation (+ (Transformation|GetActorLocation) (* (Variables|Default|GetSpeed) (Variables|Default|GetDeltaTime)) (* (* (Math|Vector|Normalize (Math|Vector|CrossProduct (Variables|Default|GetSpeed) (Transformation|GetActorRightVector))) (Math|Trig|Sin(Radians) (* (Utilities|Time|GetGameTimeinSeconds) 1e+01))) 2.0)) false false))
          (:then_2
            ;[1 1 1] Lose Tracking
            (if (!= (Variables|/Game/Blueprints/BP_Character.BP_Character_C|GetShield (Variables|Default|GetPlayer)) 2)
              (Variables|Default|SetAttracted false)
              (Variables|Default|SetMoving true)
              (Variables|Default|SetDropped true)
              (Physics|SetSimulatePhysics _collision true)
              (Physics|SetPhysicsLinearVelocity _collision (* (Variables|Default|GetSpeed) 1e+02) false "None"))))))
    (:then_2
      ;[1 1 1] Attract rings in range
      (if (Math|Boolean|ANDBoolean (== (Variables|/Game/Blueprints/BP_Character.BP_Character_C|GetShield (Variables|Default|GetPlayer)) 2) (<= (Math|Vector|VectorLength (- (Transformation|GetActorLocation (Variables|Default|GetPlayer)) (Transformation|GetActorLocation))) 512.0) (not (Variables|Default|GetDropped)))
        (Variables|Default|SetAttracted true)))))

(fn ConstructionScript)