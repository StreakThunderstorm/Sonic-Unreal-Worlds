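; Ring actor that spins its mesh around yaw every tick, with a timed lifetime when Moving is set.
; While Moving, it wakes the Collision bodies, becomes Obtainable after a short delay, later starts Fading, then destroys itself.
; Fading blinks the mesh by toggling visibility through a short Delay.
; Tick drives both the spin, which is frame-rate dependent, and the delay chains.
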(event EventTick
  (params (DeltaSeconds :type Float%20%28single-precision%29))
  (bind _ringmesh (Variables|Actor|GetRingMesh))
  (bind _returnvalue (Transformation|GetWorldRotation _ringmesh))
  (bind (_pitch _yaw _roll) (Class|KismetMathLibrary|BreakRot _returnvalue))
  (Utilities|FlowControl|Sequence
    (:then_0
      (Transformation|SetWorldRotation _ringmesh (Class|KismetMathLibrary|MakeRot _pitch (+ _yaw 5.0) _roll) false))
    (:then_1
      (if (Variables|Default|GetMoving)
        (Utilities|FlowControl|Sequence
          (:then_0
            (Class|PrimitiveComponent|WakeAllRigidBodies (Variables|Default|GetCollision))
            (Utilities|FlowControl|Delay 1.0)
            (Variables|Default|SetObtainable true)
            (Utilities|FlowControl|Delay 5.0)
            (Variables|Default|SetFading true)
            (Utilities|FlowControl|Delay 2.0)
            (Actor|DestroyActor))
          (:then_1
            (if (Variables|Default|GetFading)
              (Utilities|FlowControl|Delay 0.1)
              (Rendering|ToggleVisibility (Variables|Actor|GetRingMesh) false))))))))

(fn ConstructionScript)