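; Spline road actor that builds road meshes and collision boxes along its spline in the Construction Script.
; Random mesh variations become spline mesh segments, spaced by mesh width or, in manual mode, by chunk count and coverage.
; AddSplineMesh computes each segment's end roll from relative spline frames, supporting twisted track.
; Optional SwapVolume copies the spline offset along its up vectors and lines it with boxes on a separate collision channel.
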(event EventBeginPlay)

(event Collision|EventActorBeginOverlap
  (params (OtherActor :type Actor%20Object%20Reference)))

(fn ConstructionScript
  (bind _spline (Variables|Default|GetSpline))
  (bind _swapspline (Variables|Default|GetSwapSpline))
  (bind _meshvariations (Variables|Default|GetMeshVariations))
  (bind _meshvariations_2 (Variables|Default|GetMeshVariations))
  (bind _swapspline_2 (Variables|Default|GetSwapSpline))
  (bind _spline_2 (Variables|Default|GetSpline))
  (bind _boxsize (Variables|Default|GetBoxSize))
  (bind _returnvalue (Utilities|Array|Length _meshvariations_2))
  (bind _x (Math|Vector|BreakVector _boxsize))
  (bind _returnvalue_2 (Math|Random|RandomInteger _returnvalue))
  (bind _returnvalue_3 (* _x 2.0))
  (bind _output (Utilities|Array|Get(acopy) _meshvariations_2 _returnvalue_2))
  (Utilities|FlowControl|Sequence
    (:then_0
      (if (Variables|Default|GetManualMode)
        (Variables|Default|SetSpacing (/ (* (Spline|GetSplineLength (Variables|Default|GetSpline)) (/ (Variables|Default|GetSplineCoverage%25) 1e+02)) (Math|Conversions|ToFloat(Integer) (Variables|Default|GetNumberOfChunks))))
        (for _index (range 1 (Variables|Default|GetNumberOfChunks))
          (CallFunction|AddSplineMesh _output (* (- _index 1) (Variables|Default|GetSpacing)) (* _index (Variables|Default|GetSpacing)) (Variables|Default|GetSpacing) (Variables|Default|GetSplineCoverage%25))
          (bind _returnvalue_4 (AddComponent|AddBoxComponent false))
          (Components|Box|SetBoxExtent _returnvalue_4 (Variables|Default|GetBoxSize) true)
          (Collision|SetCollisionEnabled _returnvalue_4 "QueryAndPhysics")
          (Collision|SetCollisionObjectType _returnvalue_4 "ECC_GameTraceChannel2")
          (Collision|SetCollisionResponsetoAllChannels _returnvalue_4 "ECR_Block")
          (Transformation|SetWorldRotation _returnvalue_4 (Math|Rotator|MakeRotator (.Roll (Math|Rotator|BreakRotator (Spline|GetRotationatDistanceAlongSpline _spline_2 (* (stale _index_3) _returnvalue_3) "World"))) (.Pitch (Math|Rotator|BreakRotator (Spline|GetRotationatDistanceAlongSpline _spline_2 (* (stale _index_3) _returnvalue_3) "World"))) (.Yaw (Math|Rotator|BreakRotator (Spline|GetRotationatDistanceAlongSpline _spline_2 (* (stale _index_3) _returnvalue_3) "World")))) false false)
          (Transformation|SetWorldLocation _returnvalue_4 (+ (Spline|GetLocationatDistanceAlongSpline _spline_2 (* (stale _index_3) _returnvalue_3) "World") (* (Class|SplineComponent|GetUpVectoratDistanceAlongSpline _spline_2 (* (stale _index_3) _returnvalue_3) "World") (.Z (Math|Vector|BreakVector (Components|Box|GetScaledBoxExtent _returnvalue_4))))) false false)
          (Rendering|Debug|DrawDebugArrow :LineStart (+ (Spline|GetLocationatDistanceAlongSpline _spline_2 (* (stale _index_3) _returnvalue_3) "World") (* (Class|SplineComponent|GetUpVectoratDistanceAlongSpline _spline_2 (* (stale _index_3) _returnvalue_3) "World") (.Z (Math|Vector|BreakVector (Components|Box|GetScaledBoxExtent _returnvalue_4))))) :LineEnd (+ (+ (Spline|GetLocationatDistanceAlongSpline _spline_2 (* (stale _index_3) _returnvalue_3) "World") (* (Class|SplineComponent|GetUpVectoratDistanceAlongSpline _spline_2 (* (stale _index_3) _returnvalue_3) "World") (.Z (Math|Vector|BreakVector (Components|Box|GetScaledBoxExtent _returnvalue_4))))) (* (Math|Vector|GetRightVector _returnvalue_4) 1e+02)) :ArrowSize 1e+01 :Duration 1.0 :Thickness 5.0))
        (else
          (bind _width (CallFunction|GetMeshWidth (Utilities|Array|Get(acopy) _meshvariations (Math|Random|RandomInteger (Utilities|Array|Length _meshvariations)))))
          (Variables|Default|SetSpacing _width)
          (for _index_2 (range 1 (.ReturnValue (Math|Float|Division(WholeandRemainder) (Spline|GetSplineLength (Variables|Default|GetSpline)) (Variables|Default|GetSpacing))))
            (CallFunction|AddSplineMesh _output (* (- _index_2 1) (Variables|Default|GetSpacing)) (* _index_2 (Variables|Default|GetSpacing)) (Variables|Default|GetSpacing) 0.0))
          (for _index_3 (range 0 (.ReturnValue (Math|Float|Division(WholeandRemainder) (Spline|GetSplineLength (Variables|Default|GetSpline)) _returnvalue_3)))
            (bind _returnvalue_5 (AddComponent|AddBoxComponent false))
            (Components|Box|SetBoxExtent _returnvalue_5 (Variables|Default|GetBoxSize) true)
            (Collision|SetCollisionEnabled _returnvalue_5 "QueryAndPhysics")
            (Collision|SetCollisionObjectType _returnvalue_5 "ECC_GameTraceChannel2")
            (Collision|SetCollisionResponsetoAllChannels _returnvalue_5 "ECR_Block")
            (Transformation|SetWorldRotation _returnvalue_5 (Math|Rotator|MakeRotator (.Roll (Math|Rotator|BreakRotator (Spline|GetRotationatDistanceAlongSpline _spline_2 (* _index_3 _returnvalue_3) "World"))) (.Pitch (Math|Rotator|BreakRotator (Spline|GetRotationatDistanceAlongSpline _spline_2 (* _index_3 _returnvalue_3) "World"))) (.Yaw (Math|Rotator|BreakRotator (Spline|GetRotationatDistanceAlongSpline _spline_2 (* _index_3 _returnvalue_3) "World")))) false false)
            (Transformation|SetWorldLocation _returnvalue_5 (+ (Spline|GetLocationatDistanceAlongSpline _spline_2 (* _index_3 _returnvalue_3) "World") (* (Class|SplineComponent|GetUpVectoratDistanceAlongSpline _spline_2 (* _index_3 _returnvalue_3) "World") (.Z (Math|Vector|BreakVector (Components|Box|GetScaledBoxExtent _returnvalue_5))))) false false)
            (Rendering|Debug|DrawDebugArrow :LineStart (+ (Spline|GetLocationatDistanceAlongSpline _spline_2 (* _index_3 _returnvalue_3) "World") (* (Class|SplineComponent|GetUpVectoratDistanceAlongSpline _spline_2 (* _index_3 _returnvalue_3) "World") (.Z (Math|Vector|BreakVector (Components|Box|GetScaledBoxExtent _returnvalue_5))))) :LineEnd (+ (+ (Spline|GetLocationatDistanceAlongSpline _spline_2 (* _index_3 _returnvalue_3) "World") (* (Class|SplineComponent|GetUpVectoratDistanceAlongSpline _spline_2 (* _index_3 _returnvalue_3) "World") (.Z (Math|Vector|BreakVector (Components|Box|GetScaledBoxExtent _returnvalue_5))))) (* (Math|Vector|GetRightVector _returnvalue_5) 1e+02)) :ArrowSize 1e+01 :Duration 1.0 :Thickness 5.0)))))
    (:then_1
      (if (Variables|Default|GetSwapVolume?)
        (Utilities|FlowControl|Sequence
          (:then_0
            ;[1 1 1] Fill array with spline points
            (for _index_4 (range 0 (- (Spline|GetNumberOfSplinePoints _spline) 1))
              (Utilities|Array|Add (Variables|Default|GetSplinePoints) (Utilities|Struct|MakeSplinePoint (Math|Conversions|ToFloat(Integer) _index_4) (.location (Spline|GetTransformatSplinePoint _spline _index_4 "World" true)) (Spline|GetArriveTangentatSplinePoint _spline _index_4 "World") (Spline|GetLeaveTangentatSplinePoint _spline _index_4 "World") (.rotation (Spline|GetTransformatSplinePoint _spline _index_4 "World" true)) (.scale (Spline|GetTransformatSplinePoint _spline _index_4 "World" true)) (Class|SplineComponent|GetSplinePointType _spline _index_4)))))
          (:then_1
            (Spline|ClearSplinePoints (Variables|Default|GetSwapSpline) true))
          (:then_2
            (for (_array_element _array_index) (Variables|Default|GetSplinePoints)
              ;[1 1 1] Create Spline
              (Spline|AddSplinePointatIndex _swapspline_2 (+ (.position _array_element) (* (Math|Vector|GetUpVector (.rotation _array_element)) (Variables|Default|GetDistanceFromFloor))) _array_index "World" true)
              (Spline|SetSplinePointType _swapspline_2 _array_index (.type _array_element) false)
              (Spline|SetTangentsatSplinePoint _swapspline_2 _array_index (.arrivetangent _array_element) (.leavetangent _array_element) "World" false)
              (Class|SplineComponent|SetUpVectoratSplinePoint _swapspline_2 _array_index (Math|Vector|GetUpVector (.rotation _array_element)) "World" true)))
          (:then_3
            ;[1 1 1] Create Boxes
            (Variables|Default|SetSwapSpacing (* (Variables|Default|GetTriggerX) 2.0))
            (for _index_5 (range 0 (.ReturnValue (Math|Float|Division(WholeandRemainder) (Spline|GetSplineLength _swapspline) (Variables|Default|GetSwapSpacing))))
              (bind _returnvalue_6 (AddComponent|AddBoxComponent false))
              (Components|Box|SetBoxExtent _returnvalue_6 (Math|Vector|MakeVector (Variables|Default|GetTriggerX) (Variables|Default|GetTriggerY) (Variables|Default|GetTriggerZ)) true)
              (Collision|SetCollisionObjectType _returnvalue_6 "ECC_GameTraceChannel6")
              (Collision|SetCollisionEnabled _returnvalue_6 "QueryAndPhysics")
              (Transformation|SetWorldLocation _returnvalue_6 (Spline|GetLocationatDistanceAlongSpline _swapspline (* _index_5 (Variables|Default|GetSwapSpacing)) "World") false false)
              (Transformation|SetWorldRotation _returnvalue_6 (Spline|GetRotationatDistanceAlongSpline _swapspline (* _index_5 (Variables|Default|GetSwapSpacing)) "World") false false))))
        (else
          (Components|DestroyComponent (Variables|Default|GetSwapSpline)))))))

(fn AddSplineMesh
  (params (NewMesh :type Static%20Mesh%20Object%20Reference) (StartDistance :type Float%20%28single-precision%29) (EndDistance :type Float%20%28single-precision%29) (Spacing :type Float%20%28single-precision%29) (Coverage :type Float%20%28single-precision%29))
  (bind _spline (Variables|Default|GetSpline))
  (bind _returnvalue (Class|SplineComponent|GetScaleatDistanceAlongSpline _spline StartDistance))
  (bind _returnvalue_2 (Class|SplineComponent|GetScaleatDistanceAlongSpline _spline EndDistance))
  (bind _returnvalue_3 (Spline|GetDirectionatDistanceAlongSpline _spline EndDistance "World"))
  (bind _returnvalue_4 (Spline|GetDirectionatDistanceAlongSpline _spline StartDistance "World"))
  (bind _returnvalue_5 (Class|SplineComponent|GetUpVectoratDistanceAlongSpline _spline StartDistance "World"))
  (bind _returnvalue_6 (Class|SplineComponent|GetUpVectoratDistanceAlongSpline _spline EndDistance "World"))
  (bind _returnvalue_7 (Class|SplineComponent|GetRightVectoratDistanceAlongSpline _spline EndDistance "World"))
  (bind _returnvalue_8 (Math|Rotator|MakeRotfromZX _returnvalue_5 _returnvalue_4))
  (bind (_x _y _z) (Math|Vector|BreakVector _returnvalue))
  (bind (_x_2 _y_2 _z_2) (Math|Vector|BreakVector _returnvalue_2))
  (bind _returnvalue_9 (Class|KismetMathLibrary|NegateRotator _returnvalue_8))
  (bind _returnvalue_10 (Math|Vector|RotateVector _returnvalue_6 _returnvalue_9))
  (bind _returnvalue_11 (Math|Vector|RotateVector _returnvalue_7 _returnvalue_9))
  (bind _returnvalue_12 (Math|Vector|RotateVector _returnvalue_3 _returnvalue_9))
  (bind _returnvalue_13 (Math|Rotator|MakeRotationfromAxes _returnvalue_12 _returnvalue_11 _returnvalue_10))
  (bind _roll (Math|Rotator|BreakRotator _returnvalue_13))
  (bind _returnvalue_14 (Math|Rotator|MakeRotator _roll 0.0 0.0))
  (bind _returnvalue_15 (AddComponent|AddSplineMeshComponent true))
  (Rendering|SetCastShadow _returnvalue_15 false)
  (Components|StaticMesh|SetStaticMesh _returnvalue_15 NewMesh)
  (Collision|SetCollisionObjectType _returnvalue_15 "ECC_GameTraceChannel2")
  (Collision|SetCollisionResponsetoAllChannels _returnvalue_15 "ECR_Block")
  (Collision|SetCollisionEnabled _returnvalue_15 "QueryAndPhysics")
  (SplineMesh|SetSplineUpDir _returnvalue_15 _returnvalue_5 true)
  (Class|SplineMeshComponent|SetEndRoll _returnvalue_15 (* (Math|Trig|Acos(Degrees) (Math|Vector|DotProduct (Math|Vector|GetUpVector "0, 0, 0") (Math|Vector|GetUpVector _returnvalue_14))) (Math|Float|Sign(Float) (.Z (Math|Vector|BreakVector (Math|Vector|GetRightVector _returnvalue_14)))) -1.0) true)
  (SplineMesh|SetStartandEnd _returnvalue_15 (Spline|GetLocationatDistanceAlongSpline _spline StartDistance "World") (* _returnvalue_4 Spacing) (Spline|GetLocationatDistanceAlongSpline _spline EndDistance "World") (* _returnvalue_3 Spacing) false :!class /Script/Engine.SplineMeshComponent)
  (SplineMesh|SetStartScale _returnvalue_15 (Math|Vector2D|MakeVector2D _y _z) false :!class /Script/Engine.SplineMeshComponent)
  (SplineMesh|SetEndScale _returnvalue_15 (Math|Vector2D|MakeVector2D _y_2 _z_2) false :!class /Script/Engine.SplineMeshComponent)
  (SplineMesh|UpdateMesh _returnvalue_15)
  (return))

(fn GetMeshWidth
  (params (Mesh :type Static%20Mesh%20Object%20Reference))
  (Components|StaticMesh|SetStaticMesh (Variables|Default|GetStaticMesh) Mesh)
  (return (* (.X (Math|Vector|BreakVector (.BoxExtent (Collision|GetComponentBounds (Variables|Default|GetStaticMesh))))) 2.0)))