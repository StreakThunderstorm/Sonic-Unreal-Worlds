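; BP_SuperRing is a ring actor, named as a super ring, whose only visible behavior is a constant spin.
; BeginPlay caches the player pawn as BP_Character, though this graph never uses it.
; Tick rotates RingMesh around world yaw by a fixed step each frame, so spin speed follows frame rate.
; A 60 fps-normalized DeltaTime is computed but not applied to the rotation.
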(event EventBeginPlay
  (bind _asbp_character (Utilities|Casting|CastToBP_Character (Game|Player|GetPlayerPawn 0)))
  (Variables|Default|SetPlayer _asbp_character))

(event EventTick
  (params (DeltaSeconds :type Float%20%28single-precision%29))
  (bind _ringmesh (Variables|Actor|GetRingMesh))
  (bind _returnvalue (Transformation|GetWorldRotation _ringmesh))
  (bind (_roll _pitch _yaw) (Math|Rotator|BreakRotator _returnvalue))
  (Variables|Default|SetDeltaTime (/ DeltaSeconds 0.016))
  (Transformation|SetWorldRotation _ringmesh (Math|Rotator|MakeRotator _roll _pitch (+ _yaw -4.0)) false false))

(fn ConstructionScript)