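; Sonic character Blueprint that drives animation and visual effects from movement state such as Action, GroundSpeed and SuperForm.
; BeginPlay creates dynamic run-trail materials, then Tick maps Action to an animation enum.
; Tick also toggles and orients jump balls, spindash sphere and run trails, scaling material speeds with ground speed or spindash rev.
; Super form swaps mesh, AnimBP and sphere materials, reapplied every frame.
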(event EventBeginPlay
  (|CallParentFunction)
  (bind _returnvalue (Rendering|Material|CreateDynamicMaterialInstance (Variables|Default|GetRunTrailL) 0 "/Game/Characters/ModernSonic/Materials/SpeedrunL.SpeedrunL" :!class /Script/Engine.PrimitiveComponent))
  (Variables|Default|SetRunTrailLDynamic _returnvalue)
  (bind _returnvalue_2 (Rendering|Material|CreateDynamicMaterialInstance (Variables|Default|GetRunTrailR) 0 "/Game/Characters/ModernSonic/Materials/SpeedrunR.SpeedrunR" :!class /Script/Engine.PrimitiveComponent))
  (Variables|Default|SetRunTrailRDynamic _returnvalue_2))

(event Collision|EventActorBeginOverlap
  (params (OtherActor :type Actor%20Object%20Reference))
  (|CallParentFunction OtherActor) ; This node is disabled and will not be called.\nDrag off pins to build functionality.
)

(event EventTick
  (params (DeltaSeconds :type Float%20%28single-precision%29))
  (bind _returnvalue (Transformation|GetActorLocation))
  (bind _returnvalue_2 (Utilities|Time|GetWorldDeltaSeconds))
  (bind _returnvalue_3 (Transformation|GetActorRightVector))
  (bind _returnvalue_4 (Transformation|GetActorUpVector))
  (bind _rotinterpspeed (Variables|Default|GetRotInterpSpeed))
  (bind _jumpsphere (Variables|Default|GetJumpSphere))
  (bind _jumpsphereeffect (Variables|Default|GetJumpSphereEffect))
  (bind _jumpsphere_2 (Variables|Default|GetJumpSphere))
  (bind _jumpsphereeffect_2 (Variables|Default|GetJumpSphereEffect))
  (bind _character (Variables|Default|GetCharacter))
  (bind _runtrailholder (Variables|Default|GetRunTrailHolder))
  (bind _spindashsphere (Variables|Default|GetSpindashSphere))
  (bind _character_2 (Variables|Default|GetCharacter))
  (bind _spindashsphere_2 (Variables|Default|GetSpindashSphere))
  (bind _spindashsphere_3 (Variables|Default|GetSpindashSphere))
  (bind _character_3 (Variables|Default|GetCharacter))
  (bind _groundspeed (Variables|Default|GetGroundSpeed))
  (bind _action (Variables|Default|GetAction))
  (bind _spindashrev (Variables|Default|GetSpindashRev))
  (bind _character_4 (Variables|Default|GetCharacter))
  (bind _direction (Variables|Default|GetDirection))
  (bind _returnvalue_5 (Transformation|GetWorldRotation _character_4))
  (bind _returnvalue_6 (Transformation|GetSocketRotation _character_3 "BallRotate"))
  (bind _returnvalue_7 (Math|Float|Absolute(Float) _groundspeed))
  (bind _returnvalue_8 (* _spindashrev 2.0))
  (bind _returnvalue_9 (* _direction -1))
  (bind _returnvalue_10 (* _returnvalue_3 _returnvalue_9))
  (bind _returnvalue_11 (/ _returnvalue_7 4.0))
  (bind _returnvalue_12 (Math|Float|Clamp(Float) _returnvalue_8 5.0 1e+01))
  (bind _returnvalue_13 (Math|Rotator|MakeRotfromXZ _returnvalue_10 _returnvalue_4))
  (bind _returnvalue_14 (Math|Interpolation|RInterpTo _returnvalue_5 _returnvalue_13 _returnvalue_2 _rotinterpspeed))
  (|CallParentFunction DeltaSeconds)
  (Utilities|FlowControl|Sequence
    (:then_0
      ;[1 1 1] Set Animations
      (switch int (Variables|Default|GetAction)
        (:0
          (if (== (Variables|Default|GetGroundSpeed) 0.0)
            (Variables|Default|SetAnimations "NewEnumerator0")
            (else
              (Variables|Default|SetAnimations "NewEnumerator1"))))
        (:1
          (Variables|Default|SetAnimations "NewEnumerator2"))
        (:2
          (if (>= (Variables|Default|GetYSpeed) 0.0)
            (Variables|Default|SetAnimations "NewEnumerator10")
            (else
              (Variables|Default|SetAnimations "NewEnumerator9"))))
        (:3
          (Variables|Default|SetAnimations "NewEnumerator6"))
        (:4
          (Variables|Default|SetAnimations "NewEnumerator3"))
        (:5
          (Variables|Default|SetAnimations "NewEnumerator5"))
        (:6
          (Variables|Default|SetAnimations "NewEnumerator4"))
        (:7
          (Variables|Default|SetAnimations "NewEnumerator11"))
        (:8
          (Variables|Default|SetAnimations "NewEnumerator7"))
        (:9
          (Variables|Default|SetAnimations "NewEnumerator8"))))
    (:then_1
      ;[0 0.2982 1] Character Effects
      (Utilities|FlowControl|Sequence
        (:then_0
          ;;[1 1 1] Hide/Show Jumpshere
          (if (Math|Boolean|ORBoolean (== _action 1) (== _action 3) (== _action 7))
            (Rendering|SetVisibility _jumpsphere true false)
            (Rendering|SetVisibility _jumpsphereeffect true false)
            (else
              (Rendering|SetVisibility _jumpsphere false false)
              (Rendering|SetVisibility _jumpsphereeffect false false))))
        (:then_1
          (if (== _action 5)
            (Rendering|SetVisibility _spindashsphere true false)
            (Utilities|FlowControl|Sequence
              (:then_0
                (Rendering|SetVisibility _character_2 false false))
              (:then_1
                (goto _label Reset)))
            (else
              (Rendering|SetVisibility _spindashsphere false false)
              (Utilities|FlowControl|DoOnce false :!label _label
                (:Completed
                  (Rendering|SetVisibility _character_2 true false))))))
        (:then_2
          ;;[1 1 1] Runtrail Speed
          (Rendering|Material|SetScalarParameterValue (Variables|Default|GetRunTrailLDynamic) "Speed" _returnvalue_11 :!class /Script/Engine.MaterialInstanceDynamic)
          (Rendering|Material|SetScalarParameterValue (Variables|Default|GetRunTrailRDynamic) "Speed" _returnvalue_11 :!class /Script/Engine.MaterialInstanceDynamic))
        (:then_3
          ;;[1 1 1] Run trail visibility
          (if (Math|Boolean|ANDBoolean (== (Variables|Default|GetAction) 0) (Variables|Default|GetOnGround) (>= (Math|Float|Absolute(Float) (Variables|Default|GetGroundSpeed)) 1e+01) (not (Variables|Default|GetSuperForm)))
            (Rendering|SetVisibility _runtrailholder true true)
            (else
              (Rendering|SetVisibility _runtrailholder false true))))
        (:then_4
          ;;[1 1 1] SetJumpsphereRotation
          (Transformation|SetWorldRotation (Variables|Default|GetJumpSphereEffect) _returnvalue_6 false false)
          (Transformation|SetWorldRotation (Variables|Default|GetJumpSphere) _returnvalue_6 false false))
        (:then_5
          ;;[1 1 1] Location
          (Transformation|SetWorldLocationAndRotation (Variables|Default|GetRunTrailHolder) (+ (- (Transformation|GetActorLocation) (* (Math|Vector|GetUpVector (Variables|Default|GetCharacter)) (+ (Components|Capsule|GetScaledCapsuleHalfHeight (Variables|Default|GetCollisionCapsule)) 0.0))) (* (Transformation|GetActorForwardVector) (* (Variables|Default|GetDirection) 0.0))) _returnvalue_14 false false)
          (Transformation|SetWorldLocationAndRotation (Variables|Default|GetBoost1) (+ (Transformation|GetActorLocation) (* (Transformation|GetActorForwardVector) (* (Variables|Default|GetDirection) (+ (Components|Capsule|GetScaledCapsuleRadius (Variables|Default|GetCollisionCapsule)) 32.0)))) "0, 0, 0" false false)
          (Transformation|SetWorldLocation (Variables|Default|GetJumpSphereEffect) _returnvalue false false)
          (Transformation|SetWorldLocation (Variables|Default|GetJumpSphere) _returnvalue false false)
          (Transformation|SetWorldRotation (Variables|Default|GetSpindashSphere) _returnvalue_14 false false))))
    (:then_2
      ;[1 1 1] Super form
      (if (Variables|Default|GetSuperForm)
        (Class|SkinnedMeshComponent|SetSkeletalMesh _character "/Game/Characters/SuperSonic/SuperSonic.SuperSonic" true)
        (Components|SkeletalMesh|SetAnimInstanceClass _character "/Game/Characters/SuperSonic/ABP_SuperSonic.ABP_SuperSonic_C")
        (Rendering|Material|SetMaterial _jumpsphere_2 0 "/Game/Materials/Player/SuperSpinballMaterial.SuperSpinballMaterial")
        (Rendering|Material|SetMaterial _jumpsphereeffect_2 0 "/Game/Materials/Player/SuperSpinballEffectMaterial.SuperSpinballEffectMaterial")
        (Rendering|Material|SetMaterial _spindashsphere_2 0 "/Game/Characters/ModernSonic/Materials/SuperSonic_Spindash.SuperSonic_Spindash")
        (Rendering|Material|SetScalarParameterValueonMaterials _spindashsphere_3 "Speed" _returnvalue_12)
        (else
          (Class|SkinnedMeshComponent|SetSkeletalMesh _character "/Game/Characters/ModernSonic/ModernSonic.ModernSonic" true)
          (Components|SkeletalMesh|SetAnimInstanceClass _character "/Game/Characters/ModernSonic/ABP_ModernSonic.ABP_ModernSonic_C")
          (Rendering|Material|SetMaterial _jumpsphere_2 0 "/Game/Materials/Player/SpinballMaterial.SpinballMaterial")
          (Rendering|Material|SetMaterial _jumpsphereeffect_2 0 "/Game/Materials/Player/SpinballEffectMaterial.SpinballEffectMaterial")
          (Rendering|Material|SetMaterial _spindashsphere_2 0 "/Game/Characters/ModernSonic/Materials/SpindashMat.SpindashMat")
          (Rendering|Material|SetScalarParameterValueonMaterials _spindashsphere_3 "Speed" _returnvalue_12))))))

(fn ConstructionScript
  (|CallParentFunction))