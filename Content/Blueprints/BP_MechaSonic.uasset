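; BP_MechaSonic is the Mecha Sonic character Blueprint, driving its animation state and visual effects on top of a parent class.
; Each Tick maps Action to an animation state, using ground and vertical speed for some actions, and toggles the jump saw, spin effect and booster.
; The saws follow the BallRotate socket, and SuperForm swaps body and saw materials.
; The booster's dynamic material, created on actor overlap, receives Direction every frame.
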(event EventBeginPlay
  (|CallParentFunction) ; This node is disabled and will not be called.\nDrag off pins to build functionality.
)

(event Collision|EventActorBeginOverlap
  (params (OtherActor :type Actor%20Object%20Reference))
  (|CallParentFunction OtherActor)
  (bind _returnvalue (Rendering|Material|CreateDynamicMaterialInstance (Variables|Default|GetBooster) 0 "/Game/Materials/Player/MechaSonic_Boost.MechaSonic_Boost" :!class /Script/Engine.PrimitiveComponent))
  (Variables|Default|SetBoosterMat _returnvalue))

(event EventTick
  (params (DeltaSeconds :type Float%20%28single-precision%29))
  (bind _booster (Variables|Default|GetBooster))
  (bind _character (Variables|Default|GetCharacter))
  (bind _action (Variables|Default|GetAction))
  (bind _jumpsaw (Variables|Default|GetJumpSaw))
  (bind _jumpsaweffect (Variables|Default|GetJumpsawEffect))
  (bind _floorsensorcenterhitresult (Variables|Default|GetFloorSensorCenterHitResult))
  (bind _character_2 (Variables|Default|GetCharacter))
  (bind _jumpsaw_2 (Variables|Default|GetJumpSaw))
  (bind _jumpsaweffect_2 (Variables|Default|GetJumpsawEffect))
  (bind _character_3 (Variables|Default|GetCharacter))
  (bind _returnvalue (== _action 7))
  (bind _returnvalue_2 (Transformation|GetSocketRotation _character "BallRotate"))
  (bind (_bblockinghit _binitialoverlap _time _distance _location _impactpoint) (Collision|BreakHitResult _floorsensorcenterhitresult))
  (|CallParentFunction DeltaSeconds)
  (Utilities|FlowControl|Sequence
    (:then_0
      ;[1 1 1] Set Animations
      (switch int (Variables|Default|GetAction)
        (:0
          (if (== (Variables|Default|GetGroundSpeed) 0.0)
            (Variables|Default|SetAnimations "NewEnumerator0")
            (else
              (Variables|Default|SetAnimations "NewEnumerator1"))))
        (:1
          (Variables|Default|SetAnimations "NewEnumerator2"))
        (:2
          (if (>= (Variables|Default|GetYSpeed) 0.0)
            (Variables|Default|SetAnimations "NewEnumerator10")
            (else
              (Variables|Default|SetAnimations "NewEnumerator9"))))
        (:3
          (Variables|Default|SetAnimations "NewEnumerator6"))
        (:4
          (Variables|Default|SetAnimations "NewEnumerator3"))
        (:5
          (Variables|Default|SetAnimations "NewEnumerator5"))
        (:6
          (Variables|Default|SetAnimations "NewEnumerator4"))
        (:7
          (Variables|Default|SetAnimations "NewEnumerator11"))
        (:8
          (Variables|Default|SetAnimations "NewEnumerator7"))
        (:9
          (Variables|Default|SetAnimations "NewEnumerator8"))))
    (:then_1
      ;[0 0.2982 1] Character Effects
      (Utilities|FlowControl|Sequence
        (:then_0
          ;;[1 1 1] Hide/Show Jumpshere
          (if (or (and (== _action 1) (not (and (<= (Math|Vector|VectorLength (Math|Vector|ProjectVectorontoVector (- _impactpoint (Transformation|GetActorLocation)) (Transformation|GetActorUpVector))) (+ (Components|Capsule|GetScaledCapsuleHalfHeight (Variables|Default|GetCollisionCapsule)) 32.0)) _bblockinghit))) _returnvalue)
            (Rendering|SetVisibility _jumpsaw true false)
            (Utilities|FlowControl|Sequence
              (:then_0
                (goto _label Reset))
              (:then_1
                (Rendering|SetVisibility _character_3 false false)))
            (else
              (Rendering|SetVisibility _jumpsaw false false)
              (Utilities|FlowControl|DoOnce false :!label _label
                (:Completed
                  (Rendering|SetVisibility _character_3 true false))))))
        (:then_1
          (if _returnvalue
            (Rendering|SetVisibility _jumpsaweffect true false)
            (else
              (Rendering|SetVisibility _jumpsaweffect false false))))
        (:then_2
          (if (Math|Boolean|ANDBoolean (Variables|Default|GetOnGround) (>= (Math|Float|Absolute(Float) (Variables|Default|GetGroundSpeed)) 9.5) (== (Variables|Default|GetAction) 0))
            (Rendering|SetVisibility _booster true false)
            (else
              (Rendering|SetVisibility _booster false false))))
        (:then_3
          ;;[1 1 1] SetJumpsphereRotation
          (Transformation|SetWorldRotation (Variables|Default|GetJumpsawEffect) _returnvalue_2 false false)
          (Transformation|SetWorldRotation (Variables|Default|GetJumpSaw) _returnvalue_2 false false)
          (Rendering|Material|SetScalarParameterValue (Variables|Default|GetBoosterMat) "Direction" (Math|Conversions|ToFloat(Integer) (Variables|Default|GetDirection)) :!class /Script/Engine.MaterialInstanceDynamic))))
    (:then_2
      (if (Variables|Default|GetSuperForm)
        (Rendering|Material|SetMaterial _character_2 0 "/Game/Characters/MechaSonic/Materials/SuperMechaSonic_1002.SuperMechaSonic_1002")
        (Rendering|Material|SetMaterial _character_2 1 "/Game/Characters/MechaSonic/Materials/SuperMechaSonic_1001.SuperMechaSonic_1001")
        (Rendering|Material|SetMaterial _jumpsaw_2 0 "/Game/Characters/MechaSonic/Materials/SuperMechaSonic_Jumpsaw.SuperMechaSonic_Jumpsaw")
        (Rendering|Material|SetMaterial _jumpsaweffect_2 0 "/Game/Materials/Player/SuperSpinballEffectMaterial.SuperSpinballEffectMaterial")
        (else
          (Rendering|Material|SetMaterial _character_2 0 "/Game/Characters/MechaSonic/Materials/MechaSonic_1002.MechaSonic_1002")
          (Rendering|Material|SetMaterial _character_2 1 "/Game/Characters/MechaSonic/Materials/MechaSonic_1001.MechaSonic_1001")
          (Rendering|Material|SetMaterial _jumpsaw_2 0 "/Game/Characters/MechaSonic/Materials/MechaSonic_Jumpsaw.MechaSonic_Jumpsaw")
          (Rendering|Material|SetMaterial _jumpsaweffect_2 0 "/Game/Materials/Player/SpinballEffectMaterial.SpinballEffectMaterial"))))))

(fn ConstructionScript
  (|CallParentFunction))