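; BP_WaterVolume is a resizable water volume made of a Bounds box and a WaterPlane surface.
; The construction script sizes the box from the X, Y and Z bound variables and scales the plane to twice those values.
; It then places the plane above the actor's origin by the Z bound and applies the water material.
; The event graph holds only an empty Tick.
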(event EventTick
  (params (DeltaSeconds :type Float%20%28single-precision%29)))

(fn ConstructionScript
  (bind _returnvalue (Transformation|GetActorLocation))
  (bind _ybounds (Variables|Default|GetYBounds))
  (bind _xbounds (Variables|Default|GetXBounds))
  (bind _zbounds (Variables|Default|GetZBounds))
  (bind _waterplane (Variables|Default|GetWaterPlane))
  (bind (_x _y _z) (Math|Vector|BreakVector _returnvalue))
  (Utilities|FlowControl|Sequence
    (:then_0
      (Components|Box|SetBoxExtent (Variables|Default|GetBounds) (Math|Vector|MakeVector _xbounds _ybounds _zbounds) true))
    (:then_1
      (Transformation|SetWorldScale3D _waterplane (Math|Vector|MakeVector (* _xbounds 2.0) (* _ybounds 2.0) (* _zbounds 2.0)))
      (Transformation|SetWorldLocation _waterplane (Math|Vector|MakeVector _x _y (+ _z _zbounds)) false false)
      (Rendering|Material|SetMaterial _waterplane 0 (Variables|Default|GetWaterMaterial)))))