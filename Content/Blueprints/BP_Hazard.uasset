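; BP_Hazard is a configurable hazard actor whose HazardType selects a spike or lava mesh in the construction script.
; On Tick, spikes with PositionSwitch enabled alternate between raised and lowered targets, using a Delay as the cycle timer and playing a sound at each flip.
; VInterpTo eases the spike mesh toward the current target every frame.
; Lava has no runtime logic, and no damage handling is present.
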(event EventTick
  (params (DeltaSeconds :type Float%20%28single-precision%29))
  (bind _hazardmesh (Variables|Default|GetHazardMesh))
  (switch int (Variables|Default|GetHazardType)
    (:0
      (Utilities|FlowControl|Sequence
        (:then_0
          (if (and (Variables|Default|GetPositionSwitch) (== (Variables|Default|GetHazardType) 0))
            (if (Variables|Default|GetUp)
              (Variables|Default|SetTarget%20Location "0, 0, 0")
              (Utilities|FlowControl|Delay 3.0)
              (Audio|PlaySoundatLocation "/Game/Sounds/SpikesMove.SpikesMove" (Transformation|GetActorLocation) "0, 0, 0" 1.0 1.0 0.0 "/Game/Sounds/SoundAttenuation.SoundAttenuation")
              (Variables|Default|SetUp false)
              (else
                (Variables|Default|SetTarget%20Location "0, 0,-200.000000")
                (Utilities|FlowControl|Delay 3.0)
                (Audio|PlaySoundatLocation "/Game/Sounds/SpikesMove.SpikesMove" (Transformation|GetActorLocation) "0, 0, 0" 1.0 1.0 0.0 "/Game/Sounds/SoundAttenuation.SoundAttenuation")
                (Variables|Default|SetUp true)))))
        (:then_1
          (Transformation|SetRelativeLocation _hazardmesh (Math|Interpolation|VInterpTo (Variables|/Script/Engine.SceneComponent|GetRelativeLocation _hazardmesh) (Variables|Default|GetTarget%20Location) DeltaSeconds 25.0) false false))))))

(fn ConstructionScript
  (bind _hazardmesh (Variables|Default|GetHazardMesh))
  (bind _hazard_material (Variables|Default|GetHazard%20Material))
  (bind _hazardmesh_2 (Variables|Default|GetHazardMesh))
  (switch int (Variables|Default|GetHazardType)
    (:0
      (Components|StaticMesh|SetStaticMesh _hazardmesh "/Game/Objects/Hazards/Spikes/Spikes.Spikes") ; Spikes
      (Rendering|Material|SetMaterial _hazardmesh 0 _hazard_material))
    (:1
      (Components|StaticMesh|SetStaticMesh _hazardmesh_2 "/Game/TestMeshes/180degree100Hires.180degree100Hires") ; Lava
      (Rendering|Material|SetMaterial _hazardmesh_2 0 _hazard_material))))