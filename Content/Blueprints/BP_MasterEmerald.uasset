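; BP_MasterEmerald is the Master Emerald actor, which changes appearance once all Super Emeralds are collected.
; On BeginPlay it caches the SUWGameInstance.
; Every Tick it copies the game instance's AllSuperEmeralds flag into Awakened, then sets the Emerald mesh material to MasterEmerald when awakened or Emerald_Green otherwise.
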(event EventBeginPlay
  (bind _assuwgame_instance (Utilities|Casting|CastToSUWGameInstance (Game|GetGameInstance)))
  (Variables|Default|SetGameInstance _assuwgame_instance))

(event Collision|EventActorBeginOverlap
  (params (OtherActor :type Actor%20Object%20Reference)))

(event EventTick
  (params (DeltaSeconds :type Float%20%28single-precision%29))
  (Utilities|FlowControl|Sequence
    (:then_0
      (if (Variables|/Game/Blueprints/SUWGameInstance.SUWGameInstance_C|GetAllSuperEmeralds (Variables|Default|GetGameInstance))
        (Variables|Default|SetAwakened true)
        (else
          (Variables|Default|SetAwakened false))))
    (:then_1
      (if (Variables|Default|GetAwakened)
        (Rendering|Material|SetMaterial (Variables|Default|GetEmerald) 0 "/Game/Objects/Emeralds/Materials/MasterEmerald.MasterEmerald")
        (else
          (Rendering|Material|SetMaterial (Variables|Default|GetEmerald) 0 "/Game/Objects/Emeralds/Materials/Emerald_Green.Emerald_Green"))))))

(fn ConstructionScript)