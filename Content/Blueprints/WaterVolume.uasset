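; Water volume actor with a resizable box, a surface plane and a caustics light.
; The construction script sizes the box from the bounds variables, scales the plane onto its top face with the chosen material, and fits the light's radius and position just below the surface.
; Every tick it enables WaterEffect only while a CameraActor overlaps the volume.
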(event EventTick
  (params (DeltaSeconds :type Float%20%28single-precision%29))
  (bind _watereffect (Variables|Default|GetWaterEffect))
  (if (> (Utilities|Array|Length (Collision|GetOverlappingActors "/Script/Engine.CameraActor" :!class /Script/Engine.Actor)) 0)
    (Variables|/Script/Engine.PostProcessComponent|SetbEnabled _watereffect true)
    (else
      (Variables|/Script/Engine.PostProcessComponent|SetbEnabled _watereffect false))))

(fn ConstructionScript
  (bind _returnvalue (Transformation|GetActorLocation))
  (bind _cautsicslight (Variables|Default|GetCautsicsLight))
  (bind _ybounds (Variables|Default|GetYBounds))
  (bind _xbounds (Variables|Default|GetXBounds))
  (bind _zbounds (Variables|Default|GetZBounds))
  (bind _waterplane (Variables|Default|GetWaterPlane))
  (bind (_x _y _z) (Math|Vector|BreakVector _returnvalue))
  (bind _returnvalue_2 (* _xbounds 2.0))
  (bind _returnvalue_3 (+ _z _zbounds))
  (Utilities|FlowControl|Sequence
    (:then_0
      (Components|Box|SetBoxExtent (Variables|Default|GetBounds) (Math|Vector|MakeVector _xbounds _ybounds _zbounds) true))
    (:then_1
      (Transformation|SetWorldScale3D _waterplane (Math|Vector|MakeVector _returnvalue_2 (* _ybounds 2.0) (* _zbounds 2.0)))
      (Transformation|SetWorldLocation _waterplane (Math|Vector|MakeVector _x _y _returnvalue_3) false)
      (Rendering|Material|SetMaterial _waterplane 0 (Variables|Default|GetWaterMaterial))
      (Rendering|Lighting|SetAttenuationRadius _cautsicslight _returnvalue_2)
      (Transformation|SetWorldLocation _cautsicslight (Math|Vector|MakeVector _x _y (- _returnvalue_3 4e+01)) false))))