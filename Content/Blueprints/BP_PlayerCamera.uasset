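; Player camera actor for a Sonic-style platformer that follows BP_Character on a spring arm.
; Each tick it steps toward the player within a per-axis limit widened by a catch-up timer, then interpolates inside world bounds.
; Holding look-down lowers the view after a delay, and a nonzero spindash lag timer freezes movement and rotation.
; Yaw eases to face perpendicular to the player's movement plane.
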(event EventBeginPlay
  (Utilities|FlowControl|Sequence
    (:then_0
      ;[1 1 1] Set Player
      (bind _asbp_character (Utilities|Casting|CastToBP_Character (Game|Player|GetPlayerPawn 0)))
      (Variables|Default|SetPlayer _asbp_character)
      ;[1 1 1] Initiate camera location
      (Transformation|SetActorLocation (Transformation|GetActorLocation (Variables|Default|GetPlayer)) false true)
      (Variables|Default|SetCameraTarget (Transformation|GetActorLocation)))
    (:then_1
      (Utilities|IsValid (Variables|Default|GetPlayer)
        (:Is%20Not%20Valid
          (Actor|DestroyActor))))))

(event EventTick
  (params (DeltaSeconds :type Float%20%28single-precision%29))
  (bind _returnvalue (Transformation|GetActorLocation))
  (bind _player (Variables|Default|GetPlayer))
  (bind _player_2 (Variables|Default|GetPlayer))
  (bind _player_3 (Variables|Default|GetPlayer))
  (bind _returnvalue_2 (Transformation|GetActorLocation _player))
  (bind (_x _y _z) (Math|Vector|BreakVector _returnvalue))
  (bind _action (Variables|/Game/Blueprints/BP_Character.BP_Character_C|GetAction _player_3))
  (bind (_x_2 _y_2 _z_2) (Math|Vector|BreakVector _returnvalue_2))
  (bind _returnvalue_3 (== _action 4))
  (Variables|Default|SetDeltaTime DeltaSeconds)
  (Utilities|FlowControl|Sequence
    (:then_0
      ;[1 1 1] Calculate Camera target
      (Utilities|FlowControl|Sequence
        (:then_0
          (Variables|Default|SetTargetX (.X (Math|Vector|BreakVector (- (Math|Vector|MakeVector (+ _x_2 (Variables|Default|GetOffsetX)) _y_2 (+ _z_2 (Variables|Default|GetOffsetY))) (Transformation|GetActorLocation))))))
        (:then_1
          (Variables|Default|SetTargetY (.Z (Math|Vector|BreakVector (- (Math|Vector|MakeVector (+ _x_2 (Variables|Default|GetOffsetX)) _y_2 (+ _z_2 (Variables|Default|GetOffsetY))) (Transformation|GetActorLocation))))))
        (:then_2
          (Variables|Default|SetTarget%20Z (.Y (Math|Vector|BreakVector (- (Math|Vector|MakeVector (+ _x_2 (Variables|Default|GetOffsetX)) _y_2 (+ _z_2 (Variables|Default|GetOffsetY))) (Transformation|GetActorLocation))))))))
    (:then_1
      ;[1 1 1] Set Camera Target
      (Variables|Default|SetCameraTarget (Math|Vector|MakeVector (+ (Math|Float|Clamp(Float) (Variables|Default|GetTargetX) (* (+ (Variables|Default|GetCatchUpTimer) 64.0) -1.0) (+ (Variables|Default|GetCatchUpTimer) 64.0)) _x) (+ (Math|Float|Clamp(Float) (Variables|Default|GetTarget%20Z) (* (+ (Variables|Default|GetCatchUpTimer) 64.0) -1.0) (+ (Variables|Default|GetCatchUpTimer) 64.0)) _y) (+ (Math|Float|Clamp(Float) (Variables|Default|GetTargetY) (* (+ (Variables|Default|GetCatchUpTimer) 64.0) -1.0) (+ (Variables|Default|GetCatchUpTimer) 64.0)) _z)))
      (Variables|/Script/Engine.SpringArmComponent|SetTargetArmLength (Variables|Default|GetSpringArm) (Variables|Default|GetDistanceToPlayer)))
    (:then_2
      ;[1 1 1] Spindash Lag
      (if (> (Variables|Default|GetLagTimer) 0.0)
        (Variables|Default|SetLagTimer (Math|Float|Clamp(Float) (- (- (Variables|Default|GetLagTimer) (Variables|/Game/Blueprints/BP_Character.BP_Character_C|GetSpindashRev _player_3)) (* 1.0 (/ (Variables|Default|GetDeltaTime) 0.016))) 0.0 16.0))))
    (:then_3
      (Utilities|FlowControl|Sequence
        (:then_0
          (if _returnvalue_3
            ;[1 1 1] Look Down
            (bind _result (Math|Float|IncrementFloat (Variables|Default|GetLookupdownTimer))
              (:%20%20
                (if (>= _result 32.0)
                  (Variables|Default|SetOffsetY -256.0))))))
        (:then_1
          ;[1 1 1] Reset look up timer
          (if (not (or _returnvalue_3 (== _action 7)))
            (Variables|Default|SetLookupdownTimer 0.0)
            (Variables|Default|SetOffsetY 0.0)))))
    (:then_4
      (if (== (Variables|Default|GetLagTimer) 0.0)
        ;[1 1 1] Set Camera Position
        (Transformation|SetActorLocation (Math|Interpolation|VInterpTo (Transformation|GetActorLocation) (Math|Vector|MakeVector (Math|Float|Clamp(Float) (.X (Math|Vector|BreakVector (Variables|Default|GetCameraTarget))) (Variables|Default|GetCameraMinHorizontal) (Variables|Default|GetCameraMaxHorizontal)) (Math|Float|Clamp(Float) (.Y (Math|Vector|BreakVector (Variables|Default|GetCameraTarget))) (Variables|Default|GetCameraMinDepth) (Variables|Default|GetCameraMaxDepth)) (Math|Float|Clamp(Float) (.Z (Math|Vector|BreakVector (Variables|Default|GetCameraTarget))) (Variables|Default|GetCameraMinVertical) (Variables|Default|GetCameraMaxVertical))) (Variables|Default|GetDeltaTime) 6e+01) false true)
        ;[1 1 1] Rotate Camera
        (Transformation|SetActorRotation (Math|Interpolation|RInterpTo (Transformation|GetActorRotation) (Math|Conversions|RotationFromXVector (Math|Vector|CrossProduct (Variables|/Game/Blueprints/BP_Character.BP_Character_C|GetMovementPlaneRightVector (Variables|Default|GetPlayer)) "0, 0,1.000000")) (Variables|Default|GetDeltaTime) 4.0))))
    (:then_5
      ;[1 1 1] Catch up timer
      (if (>= (Math|Vector|VectorLength (- (Transformation|GetActorLocation (Variables|Default|GetPlayer)) (Transformation|GetActorLocation))) 128.0)
        (Variables|Default|SetCatchUpTimer (+ (Variables|Default|GetCatchUpTimer) (* 1e+01 (Variables|Default|GetDeltaTime))))
        (elif (or (<= (Variables|/Game/Blueprints/BP_Character.BP_Character_C|GetXSpeed _player_2) 6.0) (<= (Variables|/Game/Blueprints/BP_Character.BP_Character_C|GetGroundSpeed _player_2) 6.0))
          (Variables|Default|SetCatchUpTimer 0.0))))))

(fn ConstructionScript
  (Variables|/Script/Engine.SpringArmComponent|SetTargetArmLength (Variables|Default|GetSpringArm) (Variables|Default|GetDistanceToPlayer)))