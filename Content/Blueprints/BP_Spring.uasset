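; BP_Spring is a spring actor with red and yellow variants, each with its own mesh and default strength.
; The construction script picks the mesh from SpringType and sets SpringStrength unless OverrideStrength is on.
; BeginPlay stores a signed Angle of the actor's tilt against world Z, using cross products of its axis vectors and treating a zero sign as positive.
; The graphs contain no launch or overlap logic.
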(event EventBeginPlay
  (bind _returnvalue (Transformation|GetActorUpVector))
  (bind _returnvalue_2 (Transformation|GetActorRightVector))
  (bind _returnvalue_3 (Math|Vector|CrossProduct _returnvalue_2 _returnvalue))
  (bind _z (Math|Vector|BreakVector _returnvalue_3))
  (bind _returnvalue_4 (Math|Float|Sign(Float) _z))
  (Variables|Default|SetAngle (* (Math|Trig|Acos(Degrees) (Math|Vector|DotProduct (Math|Vector|CrossProduct (Transformation|GetActorRightVector) (Transformation|GetActorForwardVector)) "0, 0,1.000000")) (select (== _returnvalue_4 0.0) 1.0 _returnvalue_4))))

(fn ConstructionScript
  (bind _spring (Variables|Default|GetSpring))
  (if (Variables|Default|GetSpringType)
    (Components|StaticMesh|SetStaticMesh _spring "/Game/Objects/Springs/RedSpring.RedSpring")
    (if (not (Variables|Default|GetOverride%20Strength))
      (Variables|Default|SetSpring%20Strength 16.0))
    (else
      (Components|StaticMesh|SetStaticMesh _spring "/Game/Objects/Springs/YellowSpring.YellowSpring")
      (if (not (Variables|Default|GetOverride%20Strength))
        (Variables|Default|SetSpring%20Strength 1e+01)))))