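; Hazard actor whose type 0 is a spike trap, with the construction script assigning the Spikes mesh to HazardMesh.
; When PositionSwitch is enabled, Tick snaps the spikes between raised and lowered relative positions according to the Up flag.
; Delay nodes in Tick pace the cycle, each playing the SpikeAppear sound at the actor before flipping Up.
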(event EventTick
  (params (DeltaSeconds :type Float%20%28single-precision%29))
  (if (and (Variables|Default|GetPositionSwitch) (== (Variables|Default|GetHazardType) 0))
    (if (Variables|Default|GetUp)
      (Transformation|SetRelativeLocation (Variables|Default|GetHazardMesh) "0, 0, 0" false)
      (Utilities|FlowControl|Delay 3.0)
      (Audio|PlaySoundatLocation "/Game/Sounds/SpikeAppear.SpikeAppear" (Transformation|GetActorLocation) 1.0 1.0 0.0 "/Game/Sounds/SoundAttenuation.SoundAttenuation")
      (Variables|Default|SetUp false)
      (else
        (Transformation|SetRelativeLocation (Variables|Default|GetHazardMesh) "0,0.000000,-200.000000" false)
        (Utilities|FlowControl|Delay 3.0)
        (Audio|PlaySoundatLocation "/Game/Sounds/SpikeAppear.SpikeAppear" (Transformation|GetActorLocation) 1.0 1.0 0.0 "/Game/Sounds/SoundAttenuation.SoundAttenuation")
        (Variables|Default|SetUp true)))))

(fn ConstructionScript
  (Utilities|FlowControl|Sequence
    (:then_0
      (if (== (Variables|Default|GetHazardType) 0)
        (Components|StaticMesh|SetStaticMesh (Variables|Default|GetHazardMesh) "/Game/Objects/Spikes.Spikes")))))