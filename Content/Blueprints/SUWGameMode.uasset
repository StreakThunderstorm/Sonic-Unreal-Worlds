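; SUWGameMode is a game mode that sets up the HUD and music and handles underwater audio for the player.
; On BeginPlay it caches the BP_Character pawn, adds the SUWHUDWidget to the screen and plays a Green Hill Zone remix.
; Tick polls the pawn's Underwater flag, using a DoOnce to apply the underwater sound mix, reverb and ambient loop, undoing them on surfacing.
; Tick also copies its Lives value onto the pawn.
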(event EventBeginPlay
  (bind _asbp_character (Utilities|Casting|CastToBP_Character (Game|Player|GetPlayerPawn 0)))
  (Variables|Default|SetPlayer%20Pawn _asbp_character)
  (bind _returnvalue (UserInterface|CreateWidget "/Game/Blueprints/SUWHUDWidget.SUWHUDWidget_C"))
  (UserInterface|Viewport|AddtoPlayerScreen _returnvalue)
  (Audio|PlaySound2D "/Game/Music/▶_Sonic_The_Hedgehog_-_Green_Hill_Zone_Theme__Vau_Boy_Remix_.▶_Sonic_The_Hedgehog_-_Green_Hill_Zone_Theme__Vau_Boy_Remix_"))

(event EventTick
  (params (DeltaSeconds :type Float%20%28single-precision%29))
  (Utilities|FlowControl|Sequence
    (:then_0
      (if (Variables|/Game/Blueprints/BP_Character.BP_Character_C|GetUnderwater (Variables|Default|GetPlayer%20Pawn))
        (Utilities|FlowControl|DoOnce false :!label _label
          (:Completed
            (Class|GameplayStatics|SetBaseSoundMix "/Game/Sounds/Underwater.Underwater")
            (Class|GameplayStatics|ActivateReverbEffect "/Game/Sounds/UnderwaterReverb.UnderwaterReverb" "Underwater" 0.0 1.0)
            (bind _returnvalue (Audio|SpawnSound2D "/Game/Sounds/UnderwaterAmbient.UnderwaterAmbient"))))
        (else
          (Utilities|FlowControl|Sequence
            (:then_0
              (Class|GameplayStatics|SetBaseSoundMix "/Game/Sounds/GlobalSoundMix.GlobalSoundMix")
              (Class|GameplayStatics|DeactivateReverbEffect "Underwater")
              (if (not (== _returnvalue 0))
                (Audio|Components|Audio|Stop _returnvalue)))
            (:then_1
              (goto _label Reset))))))
    (:then_1
      (Variables|/Game/Blueprints/BP_Character.BP_Character_C|SetLives (Variables|Default|GetPlayer%20Pawn) (Variables|Default|GetLives)))))

(fn ConstructionScript)