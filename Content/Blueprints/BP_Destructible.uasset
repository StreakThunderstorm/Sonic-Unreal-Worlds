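; Destructible prop that the player can break by landing on it or rolling into it, as enabled by its JumpTop and Roll flags.
; Tick polls BP_Character's action and floor/side sensor hits, then applies fracture damage with an impulse and sound, bouncing the player on top hits.
; Breaking or fracturing relaxes collision and starts a frame-scaled timer that eventually destroys the actor.
; The construction script applies the configurable mesh and materials.
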(event OnComponentFracture(Destructible)
  (params (HitPoint :type Vector%20%28by%20ref%29 :default "0, 0, 0") (HitDirection :type Vector%20%28by%20ref%29 :default "0, 0, 0"))
  (bind _destructible (Variables|Default|GetDestructible))
  (Variables|Default|SetBroken true)
  (Collision|SetCollisionObjectType _destructible "ECC_WorldDynamic")
  (Collision|SetCollisionEnabled _destructible "QueryOnly"))

(event EventBeginPlay
  (bind _asbp_character (Utilities|Casting|CastToBP_Character (Game|Player|GetPlayerPawn 0)))
  (Variables|Default|SetPlayer _asbp_character))

(event EventTick
  (params (DeltaSeconds :type Float%20%28single-precision%29))
  (bind _returnvalue (Transformation|GetActorLocation))
  (bind _returnvalue_2 (Transformation|GetActorLocation))
  (bind _player (Variables|Default|GetPlayer))
  (bind _destructible (Variables|Default|GetDestructible))
  (bind _player_2 (Variables|Default|GetPlayer))
  (bind _player_3 (Variables|Default|GetPlayer))
  (bind _player_4 (Variables|Default|GetPlayer))
  (bind _destructible_2 (Variables|Default|GetDestructible))
  (bind _leftsensorhitresult (Variables|/Game/Blueprints/BP_Character.BP_Character_C|GetLeftSensorHitResult _player_4))
  (bind _rightsensorhitresult (Variables|/Game/Blueprints/BP_Character.BP_Character_C|GetRightSensorHitResult _player_4))
  (bind _collisioncapsule (Variables|/Game/Blueprints/BP_Character.BP_Character_C|GetCollisionCapsule _player_4))
  (bind _floorsensorcenterhitresult (Variables|/Game/Blueprints/BP_Character.BP_Character_C|GetFloorSensorCenterHitResult _player))
  (bind (_bblockinghit _binitialoverlap _time _distance _location _impactpoint _normal _impactnormal _physmat _hitactor) (Collision|BreakHitResult _floorsensorcenterhitresult))
  (bind (_bblockinghit_2 _binitialoverlap_2 _time_2 _distance_2 _location_2 _impactpoint_2 _normal_2 _impactnormal_2 _physmat_2 _hitactor_2) (Collision|BreakHitResult _leftsensorhitresult))
  (bind (_bblockinghit_3 _binitialoverlap_3 _time_3 _distance_3 _location_3 _impactpoint_3 _normal_3 _impactnormal_3 _physmat_3 _hitactor_3) (Collision|BreakHitResult _rightsensorhitresult))
  ;[1 1 1] Destroy pieces
  (Utilities|FlowControl|Sequence
    (:then_0
      (if (Variables|Default|GetBroken)
        (Variables|Default|SetDeathTimer (* (+ (Variables|Default|GetDeathTimer) 1.0) (/ DeltaSeconds 0.016)))))
    (:then_1
      (if (>= (Variables|Default|GetDeathTimer) 3.6e+03)
        (Actor|DestroyActor)))
    (:then_2
      (if (not (Variables|Default|GetBroken))
        (Utilities|FlowControl|Sequence
          (:then_0
            (if (Variables|Default|GetJumpTop)
              (switch int (Variables|/Game/Blueprints/BP_Character.BP_Character_C|GetAction (Variables|Default|GetPlayer))
                (:1
                  (if (Math|Boolean|ANDBoolean _bblockinghit (== _hitactor self) (<= (Variables|/Game/Blueprints/BP_Character.BP_Character_C|GetYSpeed _player_2) 0.0) (<= (Math|Vector|VectorLength (Math|Vector|ProjectVectorontoVector (- _impactpoint (Transformation|GetActorLocation _player_2)) (Transformation|GetActorUpVector _player_2))) (+ (Components|Capsule|GetScaledCapsuleHalfHeight (Variables|/Game/Blueprints/BP_Character.BP_Character_C|GetCollisionCapsule _player_2)) 8.0)))
                    (Class|DestructibleComponent|ApplyDamage (Variables|Default|GetDestructible) 1.0 _returnvalue _impactnormal 1e+04)
                    (Variables|Default|SetBroken true)
                    (Collision|SetCollisionObjectType (Variables|Default|GetDestructible) "ECC_WorldDynamic")
                    (Audio|PlaySoundatLocation "/Game/Sounds/LedgeBreak3.LedgeBreak3" _returnvalue)
                    (Variables|/Game/Blueprints/BP_Character.BP_Character_C|SetOnGround _player_3 false)
                    (Variables|/Game/Blueprints/BP_Character.BP_Character_C|SetYSpeed _player_3 (Variables|/Game/Blueprints/BP_Character.BP_Character_C|GetJumpStrength _player_3))
                    (Default|AirPhysics _player_3))))))
          (:then_1
            (if (Variables|Default|GetRoll)
              (switch int (Variables|/Game/Blueprints/BP_Character.BP_Character_C|GetAction (Variables|Default|GetPlayer))
                (:3
                  (Utilities|FlowControl|Sequence
                    (:then_0
                      (if (and (<= (Math|Vector|VectorLength (Math|Vector|ProjectVectorontoVector (- _impactpoint_2 (Transformation|GetActorLocation _player_4)) (Transformation|GetActorForwardVector _player_4))) (+ (Components|Capsule|GetScaledCapsuleRadius _collisioncapsule) 32.0)) (== _hitactor_2 self))
                        (Class|DestructibleComponent|ApplyDamage (Variables|Default|GetDestructible) 1.0 _returnvalue_2 (* _impactnormal_2 -1.0) 1e+04)
                        (Variables|Default|SetBroken true)
                        (Collision|SetCollisionObjectType _destructible_2 "ECC_WorldDynamic")
                        (Audio|PlaySoundatLocation "/Game/Sounds/LedgeBreak3.LedgeBreak3" _returnvalue_2)
                        (Collision|SetCollisionEnabled _destructible_2 "QueryOnly")))
                    (:then_1
                      (if (and (<= (Math|Vector|VectorLength (Math|Vector|ProjectVectorontoVector (- _impactpoint_3 (Transformation|GetActorLocation _player_4)) (Transformation|GetActorForwardVector _player_4))) (+ (Components|Capsule|GetScaledCapsuleRadius _collisioncapsule) 32.0)) (== _hitactor_3 self))
                        (Class|DestructibleComponent|ApplyDamage (Variables|Default|GetDestructible) 1.0 _returnvalue_2 (* _impactnormal_3 -1.0) 1e+04)
                        (Variables|Default|SetBroken true)
                        (Collision|SetCollisionObjectType _destructible "ECC_WorldDynamic")
                        (Audio|PlaySoundatLocation "/Game/Sounds/LedgeBreak3.LedgeBreak3" _returnvalue_2)
                        (Collision|SetCollisionEnabled _destructible "QueryOnly")))))))))))))

(fn ConstructionScript
  (bind _destructible (Variables|Default|GetDestructible))
  (Class|DestructibleComponent|SetDestructibleMesh _destructible (Variables|Default|GetDestructibleMesh))
  (Rendering|Material|SetMaterial _destructible 0 (Variables|Default|GetObject%20Material))
  (Rendering|Material|SetMaterial _destructible 1 (Variables|Default|GetFractured%20Material)))