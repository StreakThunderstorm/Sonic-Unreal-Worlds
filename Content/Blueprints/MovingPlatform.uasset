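; Moving platform actor that either oscillates in the XZ plane, swings on a chain, or stays stationary as a treadmill.
; The construction script builds chain links along the SwingRange spline for swings, or applies a speed-driven dynamic material for treadmills.
; Tick computes sine/cosine motion from frame-scaled angle steps, recording per-frame X/Y speeds and moving the mesh via PlatformPosition.
; Swings drive a pendulum angle by cosine, redrawing the spline and redistributing links each frame.
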(event EventTick
  (params (DeltaSeconds :type Float%20%28single-precision%29))
  (Variables|Default|SetDeltatime (* DeltaSeconds 6e+01))
  (Utilities|FlowControl|Sequence
    (:then_0
      (Transformation|SetWorldLocation (Variables|Default|GetPlatform) (Transformation|GetWorldLocation (Variables|Default|GetPlatformPosition)) false))
    (:then_1
      (if (not (Variables|Default|GetStationary))
        (if (Variables|Default|GetMoveOrSwing)
          (CallFunction|SwingingPlatform)
          (else
            (CallFunction|MovingPlatform)))))))

(fn ConstructionScript
  (bind _chainlink (Variables|Default|GetChainLink))
  (bind _swingrange (Variables|Default|GetSwingRange))
  (bind _returnvalue (Spline|GetSplineLength _swingrange))
  (Utilities|FlowControl|Sequence
    (:then_0
      (if (Variables|Default|GetMoveOrSwing)
        (Utilities|FlowControl|Sequence
          (:then_0
            (Transformation|SetWorldLocation (Variables|Default|GetPlatformPosition) (Class|SplineComponent|GetWorldLocationatSplinePoint _swingrange 1) false)
            (Variables|Default|SetDistanceY _returnvalue)
            (Variables|Default|SetAngleStepX 1.0)
            (if (Variables|Default|GetLeftOrRightSwing)
              (Variables|Default|SetDistanceX 9e+01)
              (else
                (Variables|Default|SetDistanceX -9e+01))))
          (:then_1
            (for _index (range 0 (.ReturnValue (Math|Float|Division(WholeandRemainder) _returnvalue (Variables|Default|GetChainWidth))))
              (bind _returnvalue_2 (AddComponent|AddStaticMeshComponent false))
              (Utilities|Array|Add _chainlink _returnvalue_2)
              (Components|StaticMesh|SetStaticMesh _returnvalue_2 (Variables|Default|GetChainMesh))
              (Transformation|SetWorldLocation _returnvalue_2 (Class|SplineComponent|GetWorldLocationatDistanceAlongSpline _swingrange (* (Variables|Default|GetChainWidth) (Math|Conversions|ToFloat(Integer) _index))) false)
              (Variables|Default|SetChainWidth (* (.X (Math|Vector|BreakVector (.Max (Components|StaticMesh|GetLocalBounds (Utilities|Array|Get(acopy) _chainlink))))) 2.0)))))
        (else
          (Components|DestroyComponent (Variables|Default|GetSwingRange)))))
    (:then_1
      (Components|StaticMesh|SetStaticMesh (Variables|Default|GetPlatform) (Variables|Default|GetPlatformMesh)))
    (:then_2
      (if (Variables|Default|GetStationary)
        (Variables|Default|SetPlatformMesh "/Game/TestMeshes/Treadmill.Treadmill")
        (bind _returnvalue_3 (Rendering|Material|CreateDynamicMaterialInstance (Variables|Default|GetPlatform) 0 "/Game/Materials/Objects/TreadmillMaterial.TreadmillMaterial" :!class /Script/Engine.PrimitiveComponent))
        (Rendering|Material|SetScalarParameterValue _returnvalue_3 "TreadmillSpeed" (Variables|Default|GetXSpeed) :!class /Script/Engine.MaterialInstanceDynamic)))))

(fn MovingPlatform
  (bind _returnvalue (Transformation|GetActorLocation))
  (bind _deltatime (Variables|Default|GetDeltatime))
  (bind (_x _y _z) (Math|Vector|BreakVector _returnvalue))
  (Utilities|FlowControl|Sequence
    (:then_0
      (Variables|Default|SetPreviousX (Variables|Default|GetCurrentX))
      (Variables|Default|SetPreviousY (Variables|Default|GetCurrentY))
      (Variables|Default|SetInitialAngleX (Math|Float|%(Float) (+ (Variables|Default|GetInitialAngleX) (* (Variables|Default|GetAngleStepX) _deltatime)) 3.6e+02))
      (Variables|Default|SetInitialAngleY (Math|Float|%(Float) (+ (Variables|Default|GetInitialAngleY) (* (Variables|Default|GetAngleStepY) _deltatime)) 3.6e+02)))
    (:then_1
      (if (Variables|Default|GetCosSinX)
        (Variables|Default|SetCurrentX (+ _x (* (Math|Trig|Sin(Degrees) (Variables|Default|GetInitialAngleX)) (Variables|Default|GetDistanceX))))
        (else
          (Variables|Default|SetCurrentX (+ _x (* (Math|Trig|Cos(Degrees) (Variables|Default|GetInitialAngleX)) (Variables|Default|GetDistanceX)))))))
    (:then_2
      (if (Variables|Default|GetCosSinY)
        (Variables|Default|SetCurrentY (+ _z (* (Math|Trig|Sin(Degrees) (Variables|Default|GetInitialAngleY)) (Variables|Default|GetDistanceY))))
        (else
          (Variables|Default|SetCurrentY (+ _z (* (Math|Trig|Cos(Degrees) (Variables|Default|GetInitialAngleY)) (Variables|Default|GetDistanceY)))))))
    (:then_3
      (Variables|Default|SetXSpeed (- (Variables|Default|GetCurrentX) (Variables|Default|GetPreviousX)))
      (Variables|Default|SetYSpeed (- (Variables|Default|GetCurrentY) (Variables|Default|GetPreviousY))))
    (:then_4
      (Transformation|SetWorldLocation (Variables|Default|GetPlatformPosition) (Math|Vector|MakeVector (Variables|Default|GetCurrentX) _y (Variables|Default|GetCurrentY)) false)))
  (return))

(fn SwingingPlatform
  (bind _returnvalue (Transformation|GetActorLocation))
  (bind _chainlink (Variables|Default|GetChainLink))
  (bind _swingrange (Variables|Default|GetSwingRange))
  (bind (_x _y _z) (Math|Vector|BreakVector _returnvalue))
  (Utilities|FlowControl|Sequence
    (:then_0
      (Variables|Default|SetPreviousX (Variables|Default|GetCurrentX))
      (Variables|Default|SetPreviousY (Variables|Default|GetCurrentY))
      (Variables|Default|SetInitialAngleX (+ (Variables|Default|GetInitialAngleX) (* (Variables|Default|GetAngleStepX) (Variables|Default|GetDeltatime))))
      (Variables|Default|SetInitialAngleY (* (Math|Trig|Cos(Degrees) (Variables|Default|GetInitialAngleX)) (Variables|Default|GetDistanceX)))
      (return))
    (:then_1
      (Variables|Default|SetCurrentX (+ _x (* (Math|Trig|Sin(Degrees) (Variables|Default|GetInitialAngleY)) (Variables|Default|GetDistanceY))))
      (return))
    (:then_2
      (Variables|Default|SetCurrentY (+ (* (- 0.0 (Math|Trig|Cos(Degrees) (Variables|Default|GetInitialAngleY))) (Variables|Default|GetDistanceY)) _z))
      (return))
    (:then_3
      (Variables|Default|SetXSpeed (- (Variables|Default|GetCurrentX) (Variables|Default|GetPreviousX)))
      (Variables|Default|SetYSpeed (- (Variables|Default|GetCurrentY) (Variables|Default|GetPreviousY)))
      (return))
    (:then_4
      (Transformation|SetWorldLocation (Variables|Default|GetPlatformPosition) (Math|Vector|MakeVector (Variables|Default|GetCurrentX) _y (Variables|Default|GetCurrentY)) false)
      (return))
    (:then_5
      (Class|SplineComponent|SetSplineWorldPoints (Variables|Default|GetSwingRange) (Utilities|Array|MakeArray (Transformation|GetWorldLocation (Variables|Default|GetPlatformStart)) (Transformation|GetWorldLocation (Variables|Default|GetPlatformPosition))))
      (for (_array_element _array_index) _chainlink
        (Transformation|SetWorldLocation _array_element (Class|SplineComponent|GetWorldLocationatDistanceAlongSpline _swingrange (* (/ (Spline|GetSplineLength _swingrange) (Math|Conversions|ToFloat(Integer) (Utilities|Array|Length _chainlink))) (Math|Conversions|ToFloat(Integer) _array_index))) false)))))