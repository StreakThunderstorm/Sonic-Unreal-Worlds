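; BP_Forceroll is an actor that toggles the player character's ForceRoll flag when the player overlaps it.
; On BeginPlay it casts the first player pawn to BP_Character and caches it.
; Each overlap by that character flips the flag and prints a ROLL ON or ROLL OFF message to screen.
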(event EventBeginPlay
  (bind _asbp_character (Utilities|Casting|CastToBP_Character (Game|Player|GetPlayerPawn 0)))
  (Variables|Default|SetPlayer _asbp_character))

(event EventTick
  (params (DeltaSeconds :type Float%20%28single-precision%29)))

(event Collision|EventActorBeginOverlap
  (params (OtherActor :type Actor%20Object%20Reference))
  (bind _player (Variables|Default|GetPlayer))
  (if (== OtherActor _player)
    (if (Variables|/Game/Blueprints/BP_Character.BP_Character_C|GetForceRoll _player)
      (Variables|/Game/Blueprints/BP_Character.BP_Character_C|SetForceRoll _player false)
      (Development|PrintString "ROLL OFF")
      (else
        (Variables|/Game/Blueprints/BP_Character.BP_Character_C|SetForceRoll _player true)
        (Development|PrintString "ROLL ON")))))

(fn ConstructionScript)