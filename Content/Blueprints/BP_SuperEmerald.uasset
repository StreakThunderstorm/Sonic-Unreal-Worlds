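; Super Emerald actor that shows one of seven colored emeralds, lit or disabled depending on whether it has been awakened.
; On BeginPlay it reads the per-color Super Emerald flags from SUWGameInstance and sets Awakened when the flag matching its EmeraldType is true.
; The construction script and every Tick both apply the color material for that type, or the disabled material while not awakened.
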(event EventBeginPlay
  (bind _assuwgame_instance (Utilities|Casting|CastToSUWGameInstance (Game|GetGameInstance)))
  (Utilities|FlowControl|Sequence
    (:then_0
      (if (Variables|/Game/Blueprints/SUWGameInstance.SUWGameInstance_C|GetSuperRedEmerald _assuwgame_instance)
        (if (== (Variables|Default|GetEmeraldType) 0)
          (Variables|Default|SetAwakened true :!label _label))))
    (:then_1
      (if (Variables|/Game/Blueprints/SUWGameInstance.SUWGameInstance_C|GetSuperYellowEmerald _assuwgame_instance)
        (if (== (Variables|Default|GetEmeraldType) 1)
          (goto _label))))
    (:then_2
      (if (Variables|/Game/Blueprints/SUWGameInstance.SUWGameInstance_C|GetSuperGreenEmerald _assuwgame_instance)
        (if (== (Variables|Default|GetEmeraldType) 2)
          (goto _label))))
    (:then_3
      (if (Variables|/Game/Blueprints/SUWGameInstance.SUWGameInstance_C|GetSuperCyanEmerald _assuwgame_instance)
        (if (== (Variables|Default|GetEmeraldType) 3)
          (goto _label))))
    (:then_4
      (if (Variables|/Game/Blueprints/SUWGameInstance.SUWGameInstance_C|GetSuperBlueEmerald _assuwgame_instance)
        (if (== (Variables|Default|GetEmeraldType) 4)
          (goto _label))))
    (:then_5
      (if (Variables|/Game/Blueprints/SUWGameInstance.SUWGameInstance_C|GetSuperPurpleEmerald _assuwgame_instance)
        (if (== (Variables|Default|GetEmeraldType) 5)
          (goto _label))))
    (:then_6
      (if (Variables|/Game/Blueprints/SUWGameInstance.SUWGameInstance_C|GetSuperSilverEmerald _assuwgame_instance)
        (if (== (Variables|Default|GetEmeraldType) 6)
          (goto _label))))))

(event Collision|EventActorBeginOverlap
  (params (OtherActor :type Actor%20Object%20Reference)))

(event EventTick
  (params (DeltaSeconds :type Float%20%28single-precision%29))
  (bind _emerald (Variables|Default|GetEmerald))
  (if (Variables|Default|GetAwakened)
    (switch int (Variables|Default|GetEmeraldType)
      (:0
        (Rendering|Material|SetMaterial _emerald 0 "/Game/Objects/Emeralds/Materials/Emerald_Red.Emerald_Red"))
      (:1
        (Rendering|Material|SetMaterial _emerald 0 "/Game/Objects/Emeralds/Materials/Emerald_Yellow.Emerald_Yellow"))
      (:2
        (Rendering|Material|SetMaterial _emerald 0 "/Game/Objects/Emeralds/Materials/Emerald_Green.Emerald_Green"))
      (:3
        (Rendering|Material|SetMaterial _emerald 0 "/Game/Objects/Emeralds/Materials/Emerald_Cyan.Emerald_Cyan"))
      (:4
        (Rendering|Material|SetMaterial _emerald 0 "/Game/Objects/Emeralds/Materials/Emerald_Blue.Emerald_Blue"))
      (:5
        (Rendering|Material|SetMaterial _emerald 0 "/Game/Objects/Emeralds/Materials/Emerald_Purple.Emerald_Purple"))
      (:6
        (Rendering|Material|SetMaterial _emerald 0 "/Game/Objects/Emeralds/Materials/Emerald_Silver.Emerald_Silver")))
    (else
      (Rendering|Material|SetMaterial (Variables|Default|GetEmerald) 0 "/Game/Objects/Emeralds/Materials/Emerald_Disabled.Emerald_Disabled"))))

(fn ConstructionScript
  (bind _emerald (Variables|Default|GetEmerald))
  (if (Variables|Default|GetAwakened)
    (switch int (Variables|Default|GetEmeraldType)
      (:0
        (Rendering|Material|SetMaterial _emerald 0 "/Game/Objects/Emeralds/Materials/Emerald_Red.Emerald_Red"))
      (:1
        (Rendering|Material|SetMaterial _emerald 0 "/Game/Objects/Emeralds/Materials/Emerald_Yellow.Emerald_Yellow"))
      (:2
        (Rendering|Material|SetMaterial _emerald 0 "/Game/Objects/Emeralds/Materials/Emerald_Green.Emerald_Green"))
      (:3
        (Rendering|Material|SetMaterial _emerald 0 "/Game/Objects/Emeralds/Materials/Emerald_Cyan.Emerald_Cyan"))
      (:4
        (Rendering|Material|SetMaterial _emerald 0 "/Game/Objects/Emeralds/Materials/Emerald_Blue.Emerald_Blue"))
      (:5
        (Rendering|Material|SetMaterial _emerald 0 "/Game/Objects/Emeralds/Materials/Emerald_Purple.Emerald_Purple"))
      (:6
        (Rendering|Material|SetMaterial _emerald 0 "/Game/Objects/Emeralds/Materials/Emerald_Silver.Emerald_Silver")))
    (else
      (Rendering|Material|SetMaterial (Variables|Default|GetEmerald) 0 "/Game/Objects/Emeralds/Materials/Emerald_Disabled.Emerald_Disabled"))))