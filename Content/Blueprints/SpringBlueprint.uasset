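; Spring actor that comes in a red or yellow variant, selected by a SpringType flag.
; The construction script sets the Spring mesh and gives the red variant a higher SpringStrength than the yellow one.
; On BeginPlay it stores the actor's pitch rotation in Angle; no launch logic appears in this Blueprint.
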(event EventBeginPlay
  (Variables|Default|SetAngle (.Pitch (Class|KismetMathLibrary|BreakRot (Transformation|GetActorRotation)))))

(fn ConstructionScript
  (bind _spring (Variables|Default|GetSpring))
  (if (Variables|Default|GetSpringType)
    (Components|StaticMesh|SetStaticMesh _spring "/Game/Objects/RedSpring.RedSpring")
    (Variables|Default|SetSpring%20Strength 3e+01)
    (else
      (Components|StaticMesh|SetStaticMesh _spring "/Game/Objects/YellowSpring.YellowSpring")
      (Variables|Default|SetSpring%20Strength 2e+01))))