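; Crumbling platform that breaks shortly after the player stands on it, then removes itself.
; Tick polls the player's center floor sensor to activate it, then advances a delta-time counter in 60 fps frame units.
; Around one second in, it plays a break sound, applies downward destructible damage and switches collision to query-only; around five seconds, it destroys the actor.
; External fractures also flag it destroyed and relax collision.
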(event OnComponentFracture(Destructible)
  (params (HitPoint :type Vector%20%28by%20ref%29 :default "0, 0, 0") (HitDirection :type Vector%20%28by%20ref%29 :default "0, 0, 0"))
  (bind _destructible (Variables|Default|GetDestructible))
  (Variables|Default|SetDestroyed true)
  (Collision|SetCollisionObjectType _destructible "ECC_WorldDynamic")
  (Collision|SetCollisionEnabled _destructible "QueryOnly"))

(event EventBeginPlay
  (bind _asbp_character (Utilities|Casting|CastToBP_Character (Game|Player|GetPlayerPawn 0)))
  (Variables|Default|SetPlayer _asbp_character))

(event Collision|EventActorBeginOverlap
  (params (OtherActor :type Actor%20Object%20Reference)))

(event EventTick
  (params (DeltaSeconds :type Float%20%28single-precision%29))
  (bind _player (Variables|Default|GetPlayer))
  (bind _destructible (Variables|Default|GetDestructible))
  (bind _floorsensorcenterhitresult (Variables|/Game/Blueprints/BP_Character.BP_Character_C|GetFloorSensorCenterHitResult _player))
  (bind (_bblockinghit _binitialoverlap _time _distance _location _impactpoint _normal _impactnormal _physmat _hitactor) (Collision|BreakHitResult _floorsensorcenterhitresult))
  (if (Variables|Default|GetActivated)
    (if (Variables|Default|GetDestroyed)
      (Utilities|FlowControl|Sequence
        (:then_0
          ;[1 1 1] Fracture Platform
          (Class|DestructibleComponent|ApplyDamage (Variables|Default|GetDestructible) 1.0 (Transformation|GetActorLocation) (* (Transformation|GetActorUpVector) -1.0) 2e+03)
          (Collision|SetCollisionObjectType _destructible "ECC_WorldDynamic")
          (Collision|SetCollisionEnabled _destructible "QueryOnly"))
        (:then_1
          (Variables|Default|SetDestructionTimer (+ (Variables|Default|GetDestructionTimer) (* (/ DeltaSeconds 0.016) 1.0))))
        (:then_2
          ;[1 1 1] Destroy actor
          (if (>= (Variables|Default|GetDestructionTimer) 3e+02)
            (Actor|DestroyActor))))
      (else
        (Utilities|FlowControl|Sequence
          (:then_0
            (Variables|Default|SetDestructionTimer (+ (Variables|Default|GetDestructionTimer) (* (/ DeltaSeconds 0.016) 1.0))))
          (:then_1
            (if (>= (Variables|Default|GetDestructionTimer) 6e+01)
              (Audio|PlaySoundatLocation "/Game/Sounds/LedgeBreak3.LedgeBreak3" (Transformation|GetActorLocation))
              (Variables|Default|SetDestroyed true))))))
    (elif (Math|Boolean|ANDBoolean _bblockinghit (== _hitactor self) (Variables|/Game/Blueprints/BP_Character.BP_Character_C|GetOnGround _player))
      (Variables|Default|SetActivated true))))

(fn ConstructionScript
  (Class|DestructibleComponent|SetDestructibleMesh (Variables|Default|GetDestructible) (Variables|Default|GetDestructibleMesh)))