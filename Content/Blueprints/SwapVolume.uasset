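; SwapVolume is a spline-shaped volume built from box collision components; what it swaps is not defined in this graph.
; The construction script steps along YSpline at twice TriggerX, adding a box at each point, aligned to the spline's position and rotation so the boxes sit end to end.
; Each box takes its extents from the Trigger variables and uses a custom collision object type with query and physics enabled.
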(fn ConstructionScript
  (bind _yspline (Variables|Default|GetYSpline))
  (Variables|Default|SetSpacing (* (Variables|Default|GetTriggerX) 2.0))
  (for _index (range 0 (.ReturnValue (Math|Float|Division(WholeandRemainder) (Spline|GetSplineLength _yspline) (Variables|Default|GetSpacing))))
    (bind _returnvalue (AddComponent|AddBoxComponent false))
    (Components|Box|SetBoxExtent _returnvalue (Math|Vector|MakeVector (Variables|Default|GetTriggerX) (Variables|Default|GetTriggerY) (Variables|Default|GetTriggerZ)) true)
    (Collision|SetCollisionObjectType _returnvalue "ECC_GameTraceChannel6")
    (Collision|SetCollisionEnabled _returnvalue "QueryAndPhysics")
    (Transformation|SetWorldLocation _returnvalue (Class|SplineComponent|GetWorldLocationatDistanceAlongSpline _yspline (* _index (Variables|Default|GetSpacing))) false)
    (Transformation|SetWorldRotation _returnvalue (Class|SplineComponent|GetWorldRotationatDistanceAlongSpline _yspline (* _index (Variables|Default|GetSpacing))) false)))