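; Follow camera actor that becomes player 0's view target and smoothly trails the CharacterPawn.
; Each tick it interpolates toward the pawn plus camera input and speed-based look-ahead offsets, which tilt with AngleRead and ease back when slow.
; A downward trace sets a minimum camera height.
; Action 50 triggers a one-shot shake and temporary depth shift; internal Y means height and Z means world Y.
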(event EventBeginPlay
  (Game|Player|SetViewTargetwithBlend (Game|GetPlayerController 0) self 0.0 "VTBlend_Linear" 0.0 false))

(event EventTick
  (params (DeltaSeconds :type Float%20%28single-precision%29))
  (bind _returnvalue (Transformation|GetActorLocation))
  (bind (_x _y _z) (Math|Vector|BreakVector _returnvalue))
  (bind _returnvalue_2 (- _z 1e+04))
  (Variables|Default|SetDeltaTime DeltaSeconds)
  (bind _ascharacterpawn_c (Utilities|Casting|CastToCharacterPawn (Game|Player|GetPlayerPawn 0)))
  (Utilities|FlowControl|Sequence
    (:then_0
      (Transformation|SetActorLocation (Math|Interpolation|VInterpTo (Transformation|GetActorLocation) (Math|Vector|MakeVector (Variables|Default|GetCurrent%20X) (Variables|Default|GetCurrent%20Z) (Variables|Default|GetCurrent%20Y)) (Utilities|Time|GetWorldDeltaSeconds) 25.0) true))
    (:then_1
      (Utilities|FlowControl|Sequence
        (:then_0
          (Variables|Default|SetTargetX (.X (Math|Vector|BreakVector (Transformation|GetActorLocation _ascharacterpawn_c)))))
        (:then_1
          (Variables|Default|SetTarget%20Z (.Y (Math|Vector|BreakVector (Transformation|GetActorLocation _ascharacterpawn_c)))))
        (:then_2
          (Variables|Default|SetTarget%20Y (.Z (Math|Vector|BreakVector (Transformation|GetActorLocation _ascharacterpawn_c)))))))
    (:then_2
      (Utilities|FlowControl|Sequence
        (:then_0
          ;[1 1 1] Interpolate Camera
          (Variables|Default|SetCurrent%20X (+ (Variables|Default|GetTargetX) (Variables|Default|GetOffset%20X) (Variables|Default|GetCameraOffsetX) (Variables|Default|GetInputOffsetX))))
        (:then_1
          (Variables|Default|SetCurrent%20Y (Math|Float|Max(Float) (+ (Variables|Default|GetTarget%20Y) (Variables|Default|GetOffset%20Y) (Variables|Default|GetCameraOffsetY) (Variables|Default|GetInputOffsetY)) (+ (Variables|Default|GetMinCameraHeight) 5e+01))))
        (:then_2
          (Variables|Default|SetCurrent%20Z (+ (Variables|Default|GetTarget%20Z) (Variables|Default|GetOffset%20Z) (Variables|Default|GetCameraOffsetZ) (Variables|Default|GetInputOffsetZ))))
        (:then_3
          (Utilities|FlowControl|Sequence
            (:then_0
              (Variables|Default|SetInputOffsetX (* (Variables|/Game/Blueprints/CharacterPawn.CharacterPawn_C|GetCameraInputAxisX _ascharacterpawn_c) 2e+02)))
            (:then_1
              (Variables|Default|SetInputOffsetY (* (Variables|/Game/Blueprints/CharacterPawn.CharacterPawn_C|GetCameraInputAxisY _ascharacterpawn_c) 2e+02)))))))
    (:then_3
      (Utilities|FlowControl|Sequence
        (:then_0
          ;[1 1 1] X Camera Move
          (if (and (< (Variables|Default|GetOffset%20X) 5e+02) (>= (Variables|/Game/Blueprints/CharacterPawn.CharacterPawn_C|GetXSpeed _ascharacterpawn_c) 1e+01))
            (Utilities|FlowControl|Sequence
              (:then_0
                (Variables|Default|SetOffset%20X (+ (* (Variables|Default|GetDeltaTime) (- (* 5e+02 (Math|Trig|Cos(Radians) (Variables|/Game/Blueprints/CharacterPawn.CharacterPawn_C|GetAngleRead _ascharacterpawn_c))) (Variables|Default|GetOffset%20X))) (Variables|Default|GetOffset%20X))))
              (:then_1
                (Variables|Default|SetOffset%20Y (+ (* (Variables|Default|GetDeltaTime) (- (* -4e+02 (Math|Trig|Sin(Radians) (Variables|/Game/Blueprints/CharacterPawn.CharacterPawn_C|GetAngleRead _ascharacterpawn_c))) (Variables|Default|GetOffset%20Y))) (Variables|Default|GetOffset%20Y)))))))
        (:then_1
          (if (and (> (Variables|Default|GetOffset%20X) -5e+02) (<= (Variables|/Game/Blueprints/CharacterPawn.CharacterPawn_C|GetXSpeed _ascharacterpawn_c) -1e+01))
            (Utilities|FlowControl|Sequence
              (:then_0
                (Variables|Default|SetOffset%20X (+ (* (Variables|Default|GetDeltaTime) (- (* -5e+02 (Math|Trig|Cos(Radians) (Variables|/Game/Blueprints/CharacterPawn.CharacterPawn_C|GetAngleRead _ascharacterpawn_c))) (Variables|Default|GetOffset%20X))) (Variables|Default|GetOffset%20X))))
              (:then_1
                (Variables|Default|SetOffset%20Y (+ (* (Variables|Default|GetDeltaTime) (- (* 4e+02 (Math|Trig|Sin(Radians) (Variables|/Game/Blueprints/CharacterPawn.CharacterPawn_C|GetAngleRead _ascharacterpawn_c))) (Variables|Default|GetOffset%20Y))) (Variables|Default|GetOffset%20Y)))))))
        (:then_2
          ;[1 1 1] X Camera Return
          (Utilities|FlowControl|Sequence
            (:then_0
              (if (and (> (Variables|Default|GetOffset%20X) 0.0) (< (Variables|/Game/Blueprints/CharacterPawn.CharacterPawn_C|GetXSpeed _ascharacterpawn_c) 1e+01))
                (Variables|Default|SetOffset%20X (+ (Variables|Default|GetOffset%20X) (* (- 0.0 (Variables|Default|GetOffset%20X)) 0.1)))))
            (:then_1
              (if (and (< (Variables|Default|GetOffset%20X) 0.0) (> (Variables|/Game/Blueprints/CharacterPawn.CharacterPawn_C|GetXSpeed _ascharacterpawn_c) -1e+01))
                (Variables|Default|SetOffset%20X (+ (Variables|Default|GetOffset%20X) (* (- 0.0 (Variables|Default|GetOffset%20X)) 0.1)))))))
        (:then_3
          (Utilities|FlowControl|Sequence
            (:then_0
              ;[1 1 1] Y Camera Move
              (if (and (< (Variables|Default|GetOffset%20Y) 4e+02) (>= (Variables|/Game/Blueprints/CharacterPawn.CharacterPawn_C|GetYSpeed _ascharacterpawn_c) 5.0))
                (Variables|Default|SetOffset%20Y (+ (* (Variables|Default|GetDeltaTime) (- 4e+02 (Variables|Default|GetOffset%20Y))) (Variables|Default|GetOffset%20Y)))))
            (:then_1
              (if (and (> (Variables|Default|GetOffset%20Y) -4e+02) (<= (Variables|/Game/Blueprints/CharacterPawn.CharacterPawn_C|GetYSpeed _ascharacterpawn_c) -5.0))
                (Variables|Default|SetOffset%20Y (+ (* (Variables|Default|GetDeltaTime) (- -4e+02 (Variables|Default|GetOffset%20Y))) (Variables|Default|GetOffset%20Y)))))
            (:then_2
              ;[1 1 1] X Camera Return
              (if (and (> (Variables|Default|GetOffset%20Y) 0.0) (< (Variables|/Game/Blueprints/CharacterPawn.CharacterPawn_C|GetYSpeed _ascharacterpawn_c) 5.0))
                (Variables|Default|SetOffset%20Y (+ (Variables|Default|GetOffset%20Y) (* (- 0.0 (Variables|Default|GetOffset%20Y)) 0.1)))))
            (:then_3
              (if (and (< (Variables|Default|GetOffset%20Y) 0.0) (> (Variables|/Game/Blueprints/CharacterPawn.CharacterPawn_C|GetYSpeed _ascharacterpawn_c) -5.0))
                (Variables|Default|SetOffset%20Y (+ (Variables|Default|GetOffset%20Y) (* (- 0.0 (Variables|Default|GetOffset%20Y)) 0.1)))))))))
    (:then_4
      (bind (_outhit _returnvalue_3) (Collision|LineTraceForObjects _returnvalue (Math|Vector|MakeVector _x _y _returnvalue_2) (Utilities|Array|MakeArray "ObjectTypeQuery8") true 0 "None"))
      (if _returnvalue_3
        (Variables|Default|SetMinCameraHeight (.Z (Math|Vector|BreakVector (.Location (Collision|BreakHitResult _outhit)))))
        (else
          (Variables|Default|SetMinCameraHeight _returnvalue_2))))
    (:then_5
      (if (== (Variables|/Game/Blueprints/CharacterPawn.CharacterPawn_C|GetAction _ascharacterpawn_c) 5e+01)
        (Utilities|FlowControl|Sequence
          (:then_0
            (Utilities|FlowControl|DoOnce false :!label _label
              (:Completed
                (Camera|PlayWorldCameraShake "/Game/Blueprints/EffectsCameraShake.EffectsCameraShake_C" (Transformation|GetActorLocation _ascharacterpawn_c) 0.0 2e+03 1.0 true)
                (Variables|Default|SetOffset%20Z -2e+02))))
          (:then_1
            (goto _label_2 Reset)))
        (else
          (Utilities|FlowControl|Sequence
            (:then_0
              (goto _label Reset))
            (:then_1
              (Utilities|FlowControl|DoOnce false :!label _label_2
                (:Completed
                  (Variables|Default|SetOffset%20Z 0.0))))))))))

(fn ConstructionScript)