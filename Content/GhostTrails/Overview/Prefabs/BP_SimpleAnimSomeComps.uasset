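; Demo prefab Blueprint that moves three mesh components together between PointA and PointB, apparently for the GhostTrails overview.
; The Construction Script caches the initial relative locations of Mesh2 and Mesh3.
; On BeginPlay, the Anim timeline plays at AnimSpeed and lerps relative locations each update.
; Mesh1 follows the interpolated point directly, while Mesh2 and Mesh3 add their cached offsets.
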(event EventBeginPlay
  (Components|Timeline|SetPlayRate (Variables|Default|GetAnim) (Variables|Default|GetAnimSpeed))
  ;[1 1 1] A > B animation
  (bind _lerp (Timeline|Anim Play)
    (:Update
      (Transformation|SetRelativeLocation (Variables|Default|GetMesh1) (Math|Vector|Lerp(Vector) (Variables|Default|GetPointA) (Variables|Default|GetPointB) _lerp) false false)
      (Transformation|SetRelativeLocation (Variables|Default|GetMesh2) (+ (Math|Vector|Lerp(Vector) (Variables|Default|GetPointA) (Variables|Default|GetPointB) _lerp) (Variables|Default|GetMesh2InitLoc)) false false)
      (Transformation|SetRelativeLocation (Variables|Default|GetMesh3) (+ (Math|Vector|Lerp(Vector) (Variables|Default|GetPointA) (Variables|Default|GetPointB) _lerp) (Variables|Default|GetMesh3InitLoc)) false false))))

(fn ConstructionScript
  (Variables|Default|SetMesh2InitLoc (Variables|/Script/Engine.SceneComponent|GetRelativeLocation (Variables|Default|GetMesh2)))
  (Variables|Default|SetMesh3InitLoc (Variables|/Script/Engine.SceneComponent|GetRelativeLocation (Variables|Default|GetMesh3))))