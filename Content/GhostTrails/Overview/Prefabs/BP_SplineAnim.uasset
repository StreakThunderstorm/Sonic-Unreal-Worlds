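; BP_SplineAnim is a prefab actor that moves a mesh along its spline path in the Ghost Trails overview content.
; Each tick it advances a normalized time value by speed and delta time, then sets the mesh's relative location from the spline at that time without constant velocity.
; Looped splines, closed in the construction script, wrap back to the start, while open ones ping-pong between ends.
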(event EventTick
  (params (DeltaSeconds :type Float%20%28single-precision%29))
  ;[1 1 1] Animating forward / backward
  (bind _output_get (Variables|Default|SetAnimVal (+ (Variables|Default|GetAnimVal) (* (Variables|Default|GetAnimSpeed) (Utilities|Time|GetWorldDeltaSeconds) (Math|Float|SelectFloat 1.0 -1.0 (Variables|Default|GetDirForward))))))
  (if (select (Variables|Default|GetDirForward) (>= _output_get 1.0) (<= _output_get 0.0))
    (if (Variables|Default|GetLoopSpline) ; If spline is looped
      (Variables|Default|SetAnimVal 0.0) ; Start from begining
      (else
        ;[1 1 1] Switch direction
        (Variables|Default|SetDirForward (not (Variables|Default|GetDirForward))))))
  ;[1 1 1] Moving on spline path by anim time
  (Transformation|SetRelativeLocation (Variables|Default|GetMesh) (Spline|GetLocationatTime (Variables|Default|GetSpline) (Variables|Default|GetAnimVal) "Local" false) false false))

(fn ConstructionScript
  (Spline|SetClosedLoop (Variables|Default|GetSpline) (Variables|Default|GetLoopSpline)))