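; BP_SimpleAnim is a simple animated prop in the GhostTrails overview content that moves its mesh between two points.
; On BeginPlay it sets a timeline's play rate from AnimSpeed and plays it, lerping the mesh's relative location from PointA to PointB.
; When Rotating is set, each timeline update also adds a fixed yaw step, so spin speed depends on frame rate.
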(event EventBeginPlay
  (Components|Timeline|SetPlayRate (Variables|Default|GetAnim) (Variables|Default|GetAnimSpeed))
  ;[1 1 1] Up/Down animation
  (bind _lerp (Timeline|Anim Play)
    (:Update
      (Transformation|SetRelativeLocation (Variables|Default|GetMesh) (Math|Vector|Lerp(Vector) (Variables|Default|GetPointA) (Variables|Default|GetPointB) _lerp) false false)
      (if (Variables|Default|GetRotating)
        (Transformation|AddRelativeRotation (Variables|Default|GetMesh) (Math|Rotator|MakeRotator 0.0 0.0 2.0) false false)))))

(fn ConstructionScript)